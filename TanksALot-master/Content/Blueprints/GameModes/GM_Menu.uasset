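; Menu game mode that manages the player lobby and launches a match.
; On begin play it shows the W_Main widget and adds player 0.
; Added players alternate between two teams via a FlipFlop, while removal uses the player number as the array index; both update the widget.
; StartGame passes the player list and a fixed team-based ruleset to the Game Instance through LoadGameMessage.
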(event EventAddPlayer
  (params (playerNumber :type Integer))
  (Utilities|FlowControl|FlipFlop
    (:A
      (Utilities|Array|Add (Variables|Default|GetactivePlayers) (Utilities|Struct|MakePlayerInfo playerNumber)))
    (:B
      (Utilities|Array|Add (Variables|Default|GetactivePlayers) (Utilities|Struct|MakePlayerInfo playerNumber 1))))
  (Default|AddPlayer (Variables|Default|GetW_mainMenu) playerNumber))

(event EventRemovePlayer
  (params (playerNumber :type Integer))
  (Utilities|Array|RemoveIndex (Variables|Default|GetactivePlayers) playerNumber)
  (Default|RemovePlayer (Variables|Default|GetW_mainMenu) playerNumber))

(event EventBeginPlay
  (bind _returnvalue (UserInterface|CreateWidget "/Game/CustomAssets/Widgets/W_Main.W_Main_C"))
  (bind _output_get (Variables|Default|SetW_mainMenu _returnvalue))
  (UserInterface|Viewport|AddtoViewport _output_get 0)
  (CallFunction|AddPlayer))

(event EventStartGame
  (Class|IInstance|LoadGame(Message) (Game|GetGameInstance) (Variables|Default|GetactivePlayers) (Utilities|Struct|MakeGamemodeInfo (Utilities|Array|Length (Variables|Default|GetactivePlayers)) 3 3e+02 0 0 0 true)))

(fn ConstructionScript)