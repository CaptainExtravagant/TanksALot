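; PayloadGameMode is the game mode for a payload game type.
; On Init it runs the parent setup, finds the first valid Payload actor in the level, stores a reference and initializes it.
; It then initializes every PayloadPathControlPoints actor in the level, so the game mode drives setup of both the payload and its path.
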(event EventInit
  (|CallParentFunction)
  (Development|PrintString "payload gm init")
  (bind _outactors (Actor|GetAllActorsOfClass "/Game/Blueprints/PayloadBPs/Payload.Payload_C"))
  ;[1 1 1] Not sure it needs to save a ref to payload, we'll see
  (bind _array_element (Utilities|Array|ForEachLoopwithBreak _outactors :!label _label)
    (:LoopBody
      (Utilities|IsValid _array_element
        (:Is%20Valid
          (Variables|Default|SetPayload _array_element)
          (goto _label Break))))
    (:Completed
      (Default|Init (Variables|Default|GetPayload))
      (bind _outactors_2 (Actor|GetAllActorsOfClass "/Game/Blueprints/PayloadBPs/PayloadPathControlPoints.PayloadPathControlPoints_C"))
      (for _array_element_2 _outactors_2
        (Default|Init _array_element_2)))))

(event EventTick
  (params (DeltaSeconds :type Float%20%28single-precision%29)))

(event EventBeginPlay
  (|CallParentFunction))

(fn ConstructionScript
  (|CallParentFunction))