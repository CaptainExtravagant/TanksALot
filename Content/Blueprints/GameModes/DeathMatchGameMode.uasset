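; Deathmatch game mode that tracks scoring per team and ends the match when a team reaches the score limit.
; Init runs the parent setup and caches the DeathMatchGameState.
; ScorePoint increments that team's Scoreboard entry and awards kill points through the ScoreManager, using the team index as player number.
; The Scoreboard count, not the awarded points, is compared to the limit to call GameOver with that team winning.
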(event EventInit
  (|CallParentFunction)
  (Development|PrintString "dm")
  (bind _asdeath_match_game_state (Utilities|Casting|CastToDeathMatchGameState (Game|GetGameState)))
  (Variables|Default|SetDeathmatchState _asdeath_match_game_state))

(event EventScorePoint
  (params (Team :type Integer))
  (Development|PrintString (Utilities|String|ToString(Integer) Team))
  (bind _result (Math|Integer|IncrementInt (Utilities|Array|Get(acopy) (Variables|/Game/Blueprints/GameModes/DeathMatchGameState.DeathMatchGameState_C|GetScoreboard (Variables|Default|GetDeathmatchState)) Team))
    (:%20%20
      (Default|AddScore (Variables|Default|GetscoreManager) Team (Utilities|Struct|BreakGamemodeInfo (Variables|Default|GetgamemodeInfo)))
      (if (== _result (.scorelimit (Variables|Default|GetgamemodeInfo)))
        (CallFunction|GameOver true Team)))))

(event EventBeginPlay
  (|CallParentFunction))

(fn ConstructionScript)