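; Base game mode for TanksALot that sets up a local multiplayer match with a shared camera and scoring.
; A one-time Init stores player and mode info, spawns a CameraManager, gathers PlayerStarts, creates missing local players and blends views to the manager's camera.
; It then spawns a ScoreManager configured with the team setting and players.
; ScorePoint and CheckWinCondition are empty stubs.
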(event Custom|SpawnPlayers
  (for (_ _array_index) (Variables|Default|GetplayersInfo)
    (Utilities|IsValid (Game|GetPlayerController _array_index)
      (:Is%20Not%20Valid
        (bind _returnvalue (Class|GameplayStatics|CreatePlayer _array_index))
        (Game|Player|SetViewTargetwithBlend _returnvalue (Variables|/Game/CustomScripts/Managers/CameraManager.CameraManager_C|Getcamera (Variables|Default|GetcameraManager)) 0.0 "VTBlend_Linear" 0.0 false))))
  (Game|Player|SetViewTargetwithBlend _returnvalue (Variables|/Game/CustomScripts/Managers/CameraManager.CameraManager_C|Getcamera (Variables|Default|GetcameraManager)) 0.0 "VTBlend_Linear" 0.0 false))

(event Custom|GetSpawnPoints
  (bind _outactors (Actor|GetAllActorsOfClass "/Script/Engine.PlayerStart"))
  (Variables|Default|SetspawnPoints _outactors))

(event EventInit
  (params (playerInfo :type Array%20of%20Player%20Info%20Structures) (gamemodeInfo :type Gamemode%20Info%20Structure))
  (if (not (Variables|Default|Getinitialised))
    (Variables|Default|SetplayersInfo playerInfo)
    (Variables|Default|SetgamemodeInfo gamemodeInfo)
    (bind _returnvalue (Game|SpawnActorfromClass "/Game/CustomScripts/Managers/CameraManager.CameraManager_C" (Math|Transform|MakeTransform "0, 0, 0") "Undefined" 0 0))
    (bind _output_get (Variables|Default|SetcameraManager _returnvalue))
    (Default|Init _output_get)
    (CallFunction|GetSpawnPoints)
    (CallFunction|SpawnPlayers)
    (bind _returnvalue_2 (Game|SpawnActorfromClass "/Game/CustomScripts/Managers/ScoreManager.ScoreManager_C" (Math|Transform|MakeTransform "0, 0, 0") "Undefined" 0 0))
    (bind _output_get_2 (Variables|Default|SetscoreManager _returnvalue_2))
    (Default|Init _output_get_2 (Utilities|Struct|BreakGamemodeInfo (Variables|Default|GetgamemodeInfo)) (Variables|Default|GetplayersInfo))))

(fn ConstructionScript)

(fn ScorePoint
  (params (Team :type Integer)))

(fn CheckWinCondition
  (params (Score :type Integer) (Team :type Integer)))