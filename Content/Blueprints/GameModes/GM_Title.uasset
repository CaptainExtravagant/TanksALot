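; Game mode for the title screen that streams in the title level and drives the main menu.
; On BeginPlay it creates the title and options widgets, hiding options and focusing the title.
; Button events swap between the two widgets, quit the game, or open the lobby level after a short delay.
; An older streaming-based transition to the lobby remains in the graph but is disconnected.
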(event Custom|Continue
  (Utilities|FlowControl|Delay 0.5)
  (Game|OpenLevel(byName) (Variables|Default|GetlobbyLevelName)))

(event Custom|Exit
  ;[1 1 1] Quit
  (Game|QuitGame 0 "Quit"))

(event EventSettingsCancel
  ;[1 1 1] Settings Button
  (Widget|SetVisibility (Variables|Default|GettitleWidget) "Visible")
  (Widget|SetVisibility (Variables|Default|GetoptionsWidget) "Hidden")
  (Class|IUI|SetFocusWidget(Message) (Variables|Default|GettitleWidget)))

(event EventQuitButton
  ;[1 1 1] Quit
  (Game|QuitGame 0 "Quit"))

(event EventSettingsButton
  ;[1 1 1] Settings Button
  (Widget|SetVisibility (Variables|Default|GettitleWidget) "Hidden")
  (Widget|SetVisibility (Variables|Default|GetoptionsWidget) "Visible")
  (Class|IUI|SetFocusWidget(Message) (Variables|Default|GetoptionsWidget)))

(event EventBeginPlay
  (Game|LoadStreamLevel(byName) (Variables|Default|GettitleLevelName) true true)
  (bind _returnvalue (UserInterface|CreateWidget "/Game/CustomAssets/Widgets/W_Title.W_Title_C"))
  (bind _output_get (Variables|Default|SettitleWidget _returnvalue))
  (UserInterface|Viewport|AddtoViewport _output_get 0)
  (bind _returnvalue_2 (UserInterface|CreateWidget "/Game/CustomAssets/Widgets/W_Options.W_Options_C"))
  (bind _output_get_2 (Variables|Default|SetoptionsWidget _returnvalue_2))
  (UserInterface|Viewport|AddtoViewport _output_get_2 0)
  (Widget|SetVisibility _output_get_2 "Hidden")
  (Class|IUI|SetFocusWidget(Message) (Variables|Default|GettitleWidget)))

(event EventPlayButton
  ;[1 1 1] Comment
  (Utilities|FlowControl|Delay 0.5)
  (Game|OpenLevel(byName) (Variables|Default|GetlobbyLevelName)))

(fn ConstructionScript)

(fn GetCurrentMenuState
  (return "NewEnumerator0"))