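; King of the Hill game mode that rotates which hill area is active during a match.
; On BeginPlay it gathers every KOTHHillArea in the level, disables them all and activates one at random, or prints a warning if none exist.
; A looping timer then disables the current hill and reactivates a random pick, which can be the same hill again.
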(event Custom|ActivateRandomHill
  (CallFunction|DeactivateCurrentHill)
  (bind _output_get (Variables|Default|SetCurrentActiveHill (Utilities|Array|Get(acopy) (Variables|Default|GetHills) (Math|Random|RandomInteger (Utilities|Array|Length (Variables|Default|GetHills))))))
  (Default|Reactivate _output_get))

(event Custom|DeactivateCurrentHill
  (bind _currentactivehill (Variables|Default|GetCurrentActiveHill)
    (:then
      (Default|Disable _currentactivehill))
    (:else)))

(event EventBeginPlay
  (|CallParentFunction)
  (bind _outactors (Actor|GetAllActorsOfClass "/Game/Blueprints/KingOfTheHillBPs/KOTHHillArea.KOTHHillArea_C"))
  (bind _output_get (Variables|Default|SetHills _outactors))
  (if (<= (Utilities|Array|Length _output_get) 0)
    (Development|PrintString "Add in hills to fight over!!")
    (else
      (for _array_element _output_get
        (Default|Disable _array_element))
      (CallFunction|ActivateRandomHill)
      (Utilities|Time|SetTimerbyEvent (delegate Custom|ActivateRandomHill) (Variables|Default|GetHillActivationTimer) true))))

(fn ConstructionScript
  (|CallParentFunction))