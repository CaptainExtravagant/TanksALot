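; Last Tank Standing game mode Blueprint that declares a win when only one tank remains.
; On PlayerKilled it counts the BP_Tank actors in the level, and if exactly one is left it calls GameOver with that tank controller's player number as the winner.
; Init only prints a debug label before running the parent's setup.
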(event EventBeginPlay
  (|CallParentFunction) ; This node is disabled and will not be called.\nDrag off pins to build functionality.
)

(event EventTick
  (params (DeltaSeconds :type Float%20%28single-precision%29)))

(event EventPlayerKilled
  (params (controller :type Controller%20Object%20Reference))
  (bind _outactors (Actor|GetAllActorsOfClass "/Game/Blueprints/Tank/BP_Tank.BP_Tank_C"))
  (if (== (Utilities|Array|Length _outactors) 1)
    (bind _aspc_tank_controller (Utilities|Casting|CastToPC_TankController (Pawn|GetController (Utilities|Array|Get(acopy) _outactors))))
    (CallFunction|GameOver true (.playernumber (Variables|/Game/Blueprints/Tank/PlayerController/PC_TankController.PC_TankController_C|GetPlayerInfo _aspc_tank_controller)))))

(event EventInit
  (Development|PrintString "last tank standing GM")
  (|CallParentFunction))

(fn ConstructionScript
  (|CallParentFunction))