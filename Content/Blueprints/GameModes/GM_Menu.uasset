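; Main menu game mode that runs the local multiplayer lobby and launches the match.
; On BeginPlay it shows the W_Main widget, creates local players with pawns and maps each BP_LobbyTank by tank number.
; Joins and leaves update the active player list, widget and matching tank, with teams assigned by player-number parity.
; StartGame passes the players and selected gamemode to the game instance to load the Sandbox level.
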(event EventAddPlayer
  (params (playerNumber :type Integer))
  (if (== (Math|Integer|%(Integer) playerNumber 2) 0)
    (Utilities|Array|Add (Variables|Default|GetactivePlayers) (Utilities|Struct|MakePlayerInfo playerNumber 1))
    (else
      (Utilities|Array|Add (Variables|Default|GetactivePlayers) (Utilities|Struct|MakePlayerInfo playerNumber))))
  (Default|AddPlayer (Variables|Default|GetW_mainMenu) playerNumber)
  (Default|AddPlayer (.Value (Utilities|Map|Find (Variables|Default|GetlobbyTanks) playerNumber)) playerNumber))

(event EventRemovePlayer
  (params (playerNumber :type Integer))
  (Utilities|Array|RemoveIndex (Variables|Default|GetactivePlayers) playerNumber)
  (Default|RemovePlayer (Variables|Default|GetW_mainMenu) playerNumber)
  (Default|RemovePlayer (.Value (Utilities|Map|Find (Variables|Default|GetlobbyTanks) playerNumber)) playerNumber))

(event EventBeginPlay
  (bind _returnvalue (UserInterface|CreateWidget "/Game/CustomAssets/Widgets/W_Main.W_Main_C"))
  (bind _output_get (Variables|Default|SetW_mainMenu _returnvalue))
  (UserInterface|Viewport|AddtoViewport _output_get 0)
  (for _index (range 0 3)
    (Class|GameplayStatics|CreatePlayer -1))
  (bind _outactors (Actor|GetAllActorsOfClass "/Game/Blueprints/Tank/BP_LobbyTank.BP_LobbyTank_C"))
  (for _array_element _outactors
    (Utilities|Map|Add (Variables|Default|GetlobbyTanks) (Variables|/Game/Blueprints/Tank/BP_LobbyTank.BP_LobbyTank_C|GettankNum _array_element) _array_element)))

(event EventStartGame
  (Class|IInstance|LoadGame(Message) (Game|GetGameInstance) (Variables|Default|GetactivePlayers) (Variables|Default|GetselectedGamemode) "Sandbox"))

(fn ConstructionScript)