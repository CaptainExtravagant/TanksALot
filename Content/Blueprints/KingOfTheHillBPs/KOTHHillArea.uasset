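; King of the Hill capture zone actor that awards points to the team holding it, and destroys itself outside that game mode.
; Box overlap events sort player-controlled tanks into per-team lists.
; Each Tick, if only one team is present, it sends that team a point via every I_Score actor, so scoring is frame-rate dependent.
; Disable and Reactivate toggle collision and spotlight; older polling logic remains unconnected.
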(event OnComponentEndOverlap(Box)
  (params (OverlappedComponent :type Primitive%20Component%20Object%20Reference) (OtherActor :type Actor%20Object%20Reference) (OtherComp :type Primitive%20Component%20Object%20Reference) (OtherBodyIndex :type Integer))
  (bind _asbp_tank (Utilities|Casting|CastToBP_Tank OtherActor))
  (bind _aspc_tank_controller (Utilities|Casting|CastToPC_TankController (Pawn|GetController _asbp_tank)))
  (switch int (.playerteam (Variables|/Game/Blueprints/Tank/PlayerController/PC_TankController.PC_TankController_C|GetPlayerInfo _aspc_tank_controller))
    (:0
      (Utilities|Array|RemoveItem (Variables|Default|GetOverlappingTanksTeam0) _asbp_tank))
    (:1
      (Utilities|Array|RemoveItem (Variables|Default|GetOverlappingTanksTeam1) _asbp_tank))))

(event OnComponentBeginOverlap(Box)
  (params (OverlappedComponent :type Primitive%20Component%20Object%20Reference) (OtherActor :type Actor%20Object%20Reference) (OtherComp :type Primitive%20Component%20Object%20Reference) (OtherBodyIndex :type Integer) (bFromSweep :type Boolean) (SweepResult :type Hit%20Result%20Structure%20%28by%20ref%29))
  (bind _asbp_tank (Utilities|Casting|CastToBP_Tank OtherActor))
  (bind _aspc_tank_controller (Utilities|Casting|CastToPC_TankController (Pawn|GetController _asbp_tank)))
  (switch int (.playerteam (Variables|/Game/Blueprints/Tank/PlayerController/PC_TankController.PC_TankController_C|GetPlayerInfo _aspc_tank_controller))
    (:0
      (Utilities|Array|AddUnique (Variables|Default|GetOverlappingTanksTeam0) _asbp_tank))
    (:1
      (Utilities|Array|AddUnique (Variables|Default|GetOverlappingTanksTeam1) _asbp_tank))))

(event Custom|Disable
  (Components|Activation|Deactivate (Variables|Default|GetDefaultSceneRoot))
  (Collision|SetCollisionEnabled (Variables|Default|GetBox) "NoCollision")
  (Rendering|Components|Light|SetIntensity (Variables|Default|GetSpotLight) 0.0))

(event Custom|Reactivate
  (Components|Activation|Activate (Variables|Default|GetDefaultSceneRoot) false)
  (Collision|SetCollisionEnabled (Variables|Default|GetBox) "QueryOnly")
  (Rendering|Components|Light|SetIntensity (Variables|Default|GetSpotLight) 7e+04))

(event EventBeginPlay
  (Utilities|Casting|CastToKingOfTheHillGameMode (Game|GetGameMode)
    (:CastFailed
      (Actor|DestroyActor))))

(event EventTick
  (params (DeltaSeconds :type Float%20%28single-precision%29))
  (if (and (> (Utilities|Array|Length (Variables|Default|GetOverlappingTanksTeam0)) 0) (not (> (Utilities|Array|Length (Variables|Default|GetOverlappingTanksTeam1)) 0)))
    (bind _outactors (Actor|GetAllActorswithInterface "/Game/CustomScripts/Interfaces/I_Score.I_Score_C"))
    (for _array_element _outactors
      (Class|IScore|AddScore(Message) _array_element 0 1))
    (elif (and (> (Utilities|Array|Length (Variables|Default|GetOverlappingTanksTeam1)) 0) (not (> (Utilities|Array|Length (Variables|Default|GetOverlappingTanksTeam0)) 0)))
      (bind _outactors_2 (Actor|GetAllActorswithInterface "/Game/CustomScripts/Interfaces/I_Score.I_Score_C"))
      (for _array_element_2 _outactors_2
        (Class|IScore|AddScore(Message) _array_element_2 1 1)))))

(fn ConstructionScript)