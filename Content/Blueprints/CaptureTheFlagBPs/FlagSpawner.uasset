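; FlagSpawner is a level-placed actor that spawns a team's flag for the Capture the Flag game mode.
; On BeginPlay it spawns a Flag at its own transform with itself and its Team passed in, then sets the flag's colour.
; It then assigns that flag to every CaptureArea belonging to another team.
; Outside CaptureTheFlagGameMode it only deactivates its root component.
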(event EventBeginPlay
  ;[1 1 1] Make sure to set the team after placing the spawner in level
  ;[1 1 1] Checks GameMode, if not CapFlag then deactivate self
  (Utilities|Casting|CastToCaptureTheFlagGameMode (Game|GetGameMode)
    (:then
      (bind _returnvalue (Game|SpawnActorfromClass "/Game/Blueprints/CaptureTheFlagBPs/Flag.Flag_C" (Transformation|GetActorTransform) "Undefined" 0 self (Variables|Default|GetTeam) 0))
      (Default|SetFlagColour _returnvalue)
      (bind _outactors (Actor|GetAllActorsOfClass "/Game/Blueprints/CaptureTheFlagBPs/CaptureArea.CaptureArea_C")) ; Theres only 2
      (for _array_element _outactors
        (if (not (== (Variables|/Game/Blueprints/CaptureTheFlagBPs/CaptureArea.CaptureArea_C|GetTeam _array_element) (Variables|Default|GetTeam)))
          (Variables|/Game/Blueprints/CaptureTheFlagBPs/CaptureArea.CaptureArea_C|SetFlag _array_element _returnvalue))))
    (:CastFailed
      (Components|Activation|Deactivate (Variables|Default|GetDefaultSceneRoot)))))

(fn ConstructionScript)