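; Capture-the-flag pickup actor that an enemy team's BP_Tank takes by overlapping it.
; On capture it marks the tank as flag carrier, drops itself 1000 units below the map to hide, and broadcasts a capture message to every I_Message widget.
; ReturnToSpawnPoint teleports it back to its FlagSpawner and clears the carrier's flag state.
; Setflagcolour picks a red or blue material from the Team value.
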(event Custom|ReturnToSpawnPoint
  (Transformation|SetActorTransform (Transformation|GetActorTransform (Variables|Default|GetFlagSpawner)) false true)
  (bind _asbp_tank (Utilities|Casting|CastToBP_Tank (Variables|Default|GetFlagBearer)))
  (Variables|/Game/Blueprints/Tank/BP_Tank.BP_Tank_C|SetdoesHaveFlag _asbp_tank false)
  (Variables|/Game/Blueprints/Tank/BP_Tank.BP_Tank_C|SetFlag _asbp_tank 0)
  (Variables|Default|SetFlagBearer 0))

(event Custom|Set%20flag%20colour
  (bind _staticmesh (Variables|Default|GetStaticMesh))
  (switch int (Variables|Default|GetTeam)
    (:0
      (Rendering|Material|SetMaterial _staticmesh 0 "/Game/CustomAssets/Materials/Flag/M_Flag_Red.M_Flag_Red"))
    (:1
      (Rendering|Material|SetMaterial _staticmesh 0 "/Game/CustomAssets/Materials/Flag/M_Flag_Red.M_Flag_Red"))
    (:2
      (Rendering|Material|SetMaterial _staticmesh 0 "/Game/CustomAssets/Materials/Flag/M_Flag_Blue.M_Flag_Blue"))))

(event Collision|EventActorBeginOverlap
  (params (OtherActor :type Actor%20Object%20Reference))
  (bind _returnvalue (Transformation|GetActorTransform))
  (bind _asbp_tank (Utilities|Casting|CastToBP_Tank OtherActor))
  (Variables|Default|SetFlagBearer _asbp_tank)
  (bind _aspc_tank_controller (Utilities|Casting|CastToPC_TankController (Pawn|GetController _asbp_tank)))
  (if (not (== (.playerteam (Variables|/Game/Blueprints/Tank/PlayerController/PC_TankController.PC_TankController_C|GetPlayerInfo _aspc_tank_controller)) (Variables|Default|GetTeam)))
    (Variables|/Game/Blueprints/Tank/BP_Tank.BP_Tank_C|SetdoesHaveFlag _asbp_tank true)
    (Variables|/Game/Blueprints/Tank/BP_Tank.BP_Tank_C|SetFlag _asbp_tank self)
    (Transformation|SetActorTransform (Math|Transform|MakeTransform (Math|Vector|MakeVector (.x (.location _returnvalue)) (.y (.location _returnvalue)) (- (.z (.location _returnvalue)) 1e+03)) (.rotation _returnvalue) (.scale _returnvalue)))
    (bind _foundwidgets (Class|WidgetBlueprintLibrary|GetAllWidgetswithInterface "/Game/CustomScripts/Interfaces/I_Message.I_Message_C" false))
    (for _array_element _foundwidgets
      (Class|IMessage|SendTextMessage(Message) _array_element (Utilities|Text|ToText(String) (Utilities|String|Append "Team" (Utilities|String|ToString(Integer) (Variables|Default|GetTeam)) "'s flag has been captured"))))))

(fn ConstructionScript)