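; CaptureArea is the team-specific scoring zone for capture the flag, tinting its spotlight by team and destroying itself outside CaptureTheFlagGameMode.
; When a tank carrying the flag overlaps it, it checks the controller's player team against its own.
; On a match, it returns the flag to its spawn point and awards that team a point through every actor implementing the I_Score interface.
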(event EventBeginPlay
  (Utilities|Casting|CastToCaptureTheFlagGameMode (Game|GetGameMode)
    (:then
      (Rendering|Components|Light|SetLightColor (Variables|Default|GetSpotLight) (Math|Color|SelectColor "(R=0.182734,G=0.000000,B=1.000000,A=1.000000)" "(R=1.000000,G=0.498109,B=0.000000,A=1.000000)" (< (Variables|Default|GetTeam) 1)) true))
    (:CastFailed
      (Actor|DestroyActor))))

(event Collision|EventActorBeginOverlap
  (params (OtherActor :type Actor%20Object%20Reference))
  (bind _asbp_tank (Utilities|Casting|CastToBP_Tank OtherActor))
  (bind _output_get (Variables|Default|SetScoringTank _asbp_tank))
  (if (Variables|/Game/Blueprints/Tank/BP_Tank.BP_Tank_C|GetHasFlag _output_get)
    (bind _aspc_tank_controller (Utilities|Casting|CastToPC_TankController (Pawn|GetController (Variables|Default|GetScoringTank))))
    (bind _output_get_2 (Variables|Default|SetScorerInfo (Variables|/Game/Blueprints/Tank/PlayerController/PC_TankController.PC_TankController_C|GetPlayerInfo _aspc_tank_controller)))
    (if (== (Variables|Default|GetTeam) (.playerteam _output_get_2))
      (if (Variables|/Game/Blueprints/Tank/BP_Tank.BP_Tank_C|GetHasFlag (Variables|Default|GetScoringTank))
        (Default|ReturntoSpawnPoint (Variables|Default|GetFlag)) ; Also sets has flag to false
        (bind _outactors (Actor|GetAllActorswithInterface "/Game/CustomScripts/Interfaces/I_Score.I_Score_C"))
        (for _array_element _outactors
          (Class|IScore|AddScore(Message) _array_element (.playerteam (Variables|Default|GetScorerInfo)) 1))))))

(fn ConstructionScript)