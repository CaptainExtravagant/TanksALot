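; BP_TrainTrack is a spline-based train track actor that builds its visible track procedurally.
; When TrackMesh is set, the construction script adds a spline mesh component for each segment between consecutive Track spline points and attaches it to the root.
; Each segment takes its start and end locations and tangents from the spline in local space, so the pieces follow the curve.
; The event graph has no runtime logic.
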(event EventBeginPlay)

(event Collision|EventActorBeginOverlap
  (params (OtherActor :type Actor%20Object%20Reference)))

(event EventTick
  (params (DeltaSeconds :type Float%20%28single-precision%29)))

(fn ConstructionScript
  (bind _track (Variables|Default|GetTrack))
  (if (Variables|Default|GetTrackMesh?)
    (for _index (range 0 (- (Spline|GetNumberOfSplinePoints (Variables|Default|GetTrack)) 2))
      (bind _returnvalue (AddComponent|AddSplineMeshComponent true (Math|Transform|MakeTransform "0, 0, 0" "0, 0, 0" "1.000000,1.000000,1.000000")))
      (Transformation|AttachComponentToComponent _returnvalue (Variables|Default|GetDefaultSceneRoot) "None" "KeepRelative" "KeepRelative" "KeepRelative" true)
      (SplineMesh|SetStartandEnd _returnvalue (.Location (Spline|GetLocationandTangentatSplinePoint _track _index "Local")) (.Tangent (Spline|GetLocationandTangentatSplinePoint _track _index "Local")) (.Location (Spline|GetLocationandTangentatSplinePoint _track (+ _index 1) "Local")) (.Tangent (Spline|GetLocationandTangentatSplinePoint _track (+ _index 1) "Local")) true :!class /Script/Engine.SplineMeshComponent))))