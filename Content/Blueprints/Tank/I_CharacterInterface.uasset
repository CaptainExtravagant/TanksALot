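; I_CharacterInterface is a Blueprint Interface in the Tank folder that defines how other objects talk to a player character.
; Input functions pass stick and left-trigger axes, weapon fire and release, and Tan-Kyo-Drift toggling.
; Other functions set player info and a UI element, kill the player, and query self and pawn, player info, health, flag possession, projectile type and power-up name.
; It holds only signatures, leaving behavior to implementers.
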(fn ILeftStickX
  (params (Axis :type Float%20%28single-precision%29)))

(fn ILeftStickY
  (params (Axis :type Float%20%28single-precision%29)))

(fn IRightStickX
  (params (Axis :type Float%20%28single-precision%29)))

(fn IRightStickY
  (params (Axis :type Float%20%28single-precision%29)))

(fn IWeaponFire)

(fn ITan-Kyo-DriftEnabled)

(fn IWeaponReleased)

(fn ITan-Kyo-DriftDisabled)

(fn SetPlayerInfo
  (params (playerInfo :type Player%20Info%20Structure)))

(fn IKillPlayer)

(fn LLeftTrigger
  (params (axis :type Float%20%28single-precision%29)))

(fn GetSelfandPawn
  (return 0 0))

(fn GetPlayerInfo
  (return ""))

(fn GetCurrentHealth
  (return 0.0))

(fn GetMaxHealth
  (return 0.0))

(fn HasFlag
  (return false))

(fn GetCurrentProjectileType
  (return 0))

(fn GetCurrentPowerUpName
  (return "None"))

(fn SetUiElement
  (params (ui :type Widget%20Object%20Reference)))