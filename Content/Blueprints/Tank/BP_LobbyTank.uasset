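; BP_LobbyTank is a lobby display tank tied to a player slot through TankNum, appearing when that player is added.
; AddPlayer shows the Transform component and its children and enables physics when the number matches.
; RemovePlayer hides it, stops physics and returns the actor to StartPos.
; BeginPlay caches StartPos and reuses that removal path to start hidden; ChangeModel is an empty stub.
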(event Custom|ChangeModel)

(event EventBeginPlay
  (bind _transform (Variables|Default|GetTransform))
  (Variables|Default|SetstartPos (Transformation|GetActorLocation))
  (Rendering|SetVisibility _transform false true)
  (Physics|SetSimulatePhysics _transform false)
  (Transformation|SetActorLocation (Variables|Default|GetstartPos) false false))

(event Collision|EventActorBeginOverlap
  (params (OtherActor :type Actor%20Object%20Reference)))

(event EventTick
  (params (DeltaSeconds :type Float%20%28single-precision%29)))

(event EventAddPlayer
  (params (playerNumber :type Integer))
  (bind _transform (Variables|Default|GetTransform))
  (if (== playerNumber (Variables|Default|GettankNum))
    (Rendering|SetVisibility _transform true true)
    (Physics|SetSimulatePhysics _transform true)))

(event EventRemovePlayer
  (params (playerNumber :type Integer))
  (bind _transform (Variables|Default|GetTransform))
  (if (== playerNumber (Variables|Default|GettankNum))
    (Rendering|SetVisibility _transform false true)
    (Physics|SetSimulatePhysics _transform false)
    (Transformation|SetActorLocation (Variables|Default|GetstartPos) false false)))

(fn ConstructionScript)