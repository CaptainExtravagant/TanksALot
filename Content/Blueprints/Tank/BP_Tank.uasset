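; Player tank pawn with a separately spawned turret, timer-driven firing, timed power-ups and health.
; Sticks set hull and turret headings interpolated on Tick, while the trigger drives force on Base, with Root following and a downward trace aligning to slopes.
; Power-ups change projectile type, speed, health or shield invincibility, and LazorSloMo temporarily slows movement and turret turning.
; Death returns any carried flag, notifies the controller of the killer and destroys the turret.
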(event Custom|SpeedPowerUp
  ;[1 0.545 0] Speed boost
  (Variables|Default|SetTankSpeed (* (Variables|Default|GetTankSpeed) 2.0))
  (Utilities|FlowControl|Delay (Variables|Default|GetPowerUpTimer))
  (Variables|Default|SetTankSpeed (Utilities|GetClassDefaults (Utilities|GetClass self)))
  (Variables|Default|SetPoweredUp? false))

(event Custom|ShieldPowerUp
  (params (EffectDuration :type Float%20%28single-precision%29))
  (bind _shieldsphere (Variables|Default|GetShieldSphere))
  ;[1 0.545 0] Shield Power-Up
  (Variables|Default|SetInvincible? true)
  (Utilities|Time|SetTimerbyEvent (delegate Custom|ShieldOver) EffectDuration)
  (Rendering|SetVisibility _shieldsphere true false)
  (Collision|SetCollisionResponsetoChannel _shieldsphere "ECC_GameTraceChannel3" "ECR_Block"))

(event Custom|SplitShotPowerUp
  (params (Timer :type Float%20%28single-precision%29))
  (CallFunction|SetProjectileType "/Game/Blueprints/Tank/Projectiles/BP_ProjectileSplitShot.BP_ProjectileSplitShot_C" Timer))

(event Custom|RepairPowerUp
  (params (AmountRepaired :type Float%20%28single-precision%29))
  (CallFunction|AddHealth AmountRepaired))

(event Custom|ShieldOver
  (bind _shieldsphere (Variables|Default|GetShieldSphere))
  ;[1 0.545 0] Shield Power-Up
  (Variables|Default|SetInvincible? false)
  (Variables|Default|SetPoweredUp? false)
  (Rendering|SetVisibility _shieldsphere false false)
  (Collision|SetCollisionResponsetoChannel _shieldsphere "ECC_GameTraceChannel3" "ECR_Ignore"))

(event Custom|SetPowerUpTimer
  (Utilities|Time|SetTimerbyEvent (delegate Custom|ResetPowerUp) (Variables|Default|GetPowerUpTimer)))

(event Custom|ResetPowerUp
  (Variables|Default|SetPoweredUp? false))

(event Custom|RevertSpeed
  (bind _self self)
  (bind _returnvalue (Utilities|GetClass _self))
  (bind (_turret_turn_speed _tankspeed) (Utilities|GetClassDefaults _returnvalue))
  (Variables|Default|SetTurret%20Turn%20Speed _turret_turn_speed)
  (Variables|Default|SetTankSpeed _tankspeed)
  (Utilities|FlowControl|DoOnce false) ; enters at Reset
)

(event Custom|ResetFire
  ;[0.1611 1 0.08185] Weapon fire
  (Variables|Default|SetWeaponFireCooldown false))

(event Custom|HandleSlopes
  (bind _base (Variables|Default|GetBase))
  (bind _returnvalue (Transformation|GetWorldLocation _base))
  ;[1 1 1] Handle Slopes
  (bind _outhit (Collision|LineTraceByChannel _returnvalue (- _returnvalue (* (Math|Vector|GetUpVector _base) 1e+02)) "TraceTypeQuery1" false 0 "Persistent"))
  (Transformation|SetWorldRotation (Variables|Default|GetBase) (Math|Rotator|MakeRotator (.Roll (Math|Rotator|BreakRotator (Math|Rotator|MakeRotfromXZ (Transformation|GetActorForwardVector) (.ImpactNormal (Collision|BreakHitResult _outhit))))) (.Pitch (Math|Rotator|BreakRotator (Class|KismetMathLibrary|MakeRotfromYZ (Transformation|GetActorRightVector) (.ImpactNormal (Collision|BreakHitResult _outhit))))) (.Yaw (Math|Rotator|BreakRotator (Transformation|GetActorRotation)))) false false)
  (Transformation|SetWorldRotation (Variables|/Script/Engine.Actor|GetRootComponent (Variables|Default|GetTurret)) (Math|Rotator|MakeRotator (.Roll (Math|Rotator|BreakRotator (Math|Rotator|MakeRotator (.Roll (Math|Rotator|BreakRotator (Math|Rotator|MakeRotfromXZ (Transformation|GetActorForwardVector) (.ImpactNormal (Collision|BreakHitResult _outhit))))) (.Pitch (Math|Rotator|BreakRotator (Class|KismetMathLibrary|MakeRotfromYZ (Transformation|GetActorRightVector) (.ImpactNormal (Collision|BreakHitResult _outhit))))) (.Yaw (Math|Rotator|BreakRotator (Transformation|GetActorRotation)))))) (.Pitch (Math|Rotator|BreakRotator (Math|Rotator|MakeRotator (.Roll (Math|Rotator|BreakRotator (Math|Rotator|MakeRotfromXZ (Transformation|GetActorForwardVector) (.ImpactNormal (Collision|BreakHitResult _outhit))))) (.Pitch (Math|Rotator|BreakRotator (Class|KismetMathLibrary|MakeRotfromYZ (Transformation|GetActorRightVector) (.ImpactNormal (Collision|BreakHitResult _outhit))))) (.Yaw (Math|Rotator|BreakRotator (Transformation|GetActorRotation)))))) 0.0) false false))

(event Custom|AddHealth
  (params (Amount :type Float%20%28single-precision%29))
  ;[0.1611 1 0.08185] Health and Damage
  (Variables|Default|SetCurrentHealth (Math|Float|Clamp(Float) (+ Amount (Variables|Default|GetCurrentHealth)) 0.0 (Variables|Default|GetMaxHealth))))

(event Custom|PawnDeath
  (bind _lastattackedby (Variables|Default|GetLastAttackedBy))
  ;[0.1611 1 0.08185] Health and Damage
  (Development|PrintString "pawn died")
  (if (Variables|Default|GetHasFlag)
    (Development|PrintString "died with flag")
    (Default|ReturntoSpawnPoint (Variables|Default|GetFlag)))
  (if (Utilities|IsValid _lastattackedby)
    (bind _aspc_tank_controller (Utilities|Casting|CastToPC_TankController (Pawn|GetController _lastattackedby))))
  (Default|Killed (.AsPC%20Tank%20Controller (Utilities|Casting|CastToPC_TankController (Pawn|GetController))) _aspc_tank_controller)
  (Actor|DestroyActor (Variables|Default|GetTurret)))

(event Custom|LazorSloMo
  (params (Duration :type Float%20%28single-precision%29))
  (Utilities|FlowControl|DoOnce false
    (:Completed
      (Variables|Default|SetTankSpeed (/ (Variables|Default|GetTankSpeed) 2.0))
      (Variables|Default|SetPreviousTurretTurnSpeed (Variables|Default|GetTurret%20Turn%20Speed))
      (Variables|Default|SetTurret%20Turn%20Speed (/ (Variables|Default|GetTurret%20Turn%20Speed) 2e+01))
      (Utilities|Time|SetTimerbyEvent (delegate Custom|RevertSpeed) Duration))))

(event Custom|WeaponFire
  (bind _turret (Variables|Default|GetTurret))
  (bind _firepoint (Variables|/Game/Blueprints/Tank/BP_Turret.BP_Turret_C|GetFirePoint _turret))
  (bind _returnvalue (Transformation|GetWorldTransform _firepoint))
  ;[0.1611 1 0.08185] Weapon fire
  (bind _returnvalue_2 (Game|SpawnActorfromClass (Variables|Default|GetProjectileType) (Math|Transform|MakeTransform (.location _returnvalue) (.rotation _returnvalue) (.scale _returnvalue)) "Undefined" 0 self))
  (if (Utilities|DoesObjectImplementInterface _returnvalue_2 "/Game/Blueprints/PickUps/I_SplitShot.I_SplitShot_C")
    (bind _asbp_projectile_split_shot (Utilities|Casting|CastToBP_ProjectileSplitShot _returnvalue_2))
    (Default|SpawnSplitProjectiles _asbp_projectile_split_shot (Variables|Default|GetPreviousProjectileType)))
  (Variables|Default|SetWeaponFireCooldown true)
  (Utilities|Time|SetTimerbyEvent (delegate Custom|ResetFire) (Variables|Default|GetFireDelay)))

(event Custom|SetProjectileType
  (params (NewProjectileType :type BP%20Projectile%20Base%20Class%20Reference) (Time :type Float%20%28single-precision%29))
  ;[1 1 1] Projectile PickUp timer
  (if (== (Variables|Default|GetProjectileType) "/Game/Blueprints/Tank/Projectiles/BP_ProjectileSplitShot.BP_ProjectileSplitShot_C")
    _
    (else
      (Variables|Default|SetPreviousProjectileType (Variables|Default|GetProjectileType))))
  (Variables|Default|SetProjectileType NewProjectileType)
  (Utilities|Time|SetTimerbyEvent (delegate Custom|RevertProjectileType) Time))

(event Custom|RevertProjectileType
  ;[1 1 1] Projectile PickUp timer
  (if (== (Variables|Default|GetProjectileType) "/Game/Blueprints/Tank/Projectiles/BP_ProjectileSplitShot.BP_ProjectileSplitShot_C")
    (Variables|Default|SetPoweredUp? false)
    (CallFunction|SetProjectileType (Variables|Default|GetPreviousProjectileType) 5.0) ; Probably shouldn't be hard coded
    (else
      (Variables|Default|SetProjectileType (Utilities|GetClassDefaults (Utilities|GetClass self))))))

(event EventILeftStickY
  (params (Axis :type Float%20%28single-precision%29))
  ;[1 1 1] Left Stick
  (if (!= (Math|Float|Absolute(Float) Axis) 0.0)
    (Variables|Default|SetRotationalVector (Math|Vector|MakeVector Axis (stale EventILeftStickX Axis) 0.0))))

(event EventTick
  (params (DeltaSeconds :type Float%20%28single-precision%29))
  ;[1 1 1] Tick
  (bind _pivot (Variables|/Game/Blueprints/Tank/BP_Turret.BP_Turret_C|GetPivot (Variables|Default|GetTurret))
    (:then
      (Transformation|SetRelativeRotation _pivot (Math|Interpolation|RInterpTo (Variables|/Script/Engine.SceneComponent|GetRelativeRotation _pivot) (Math|Conversions|RotationFromXVector (Math|Vector|Normalize (Variables|Default|GetTurretRotationalVector))) (Utilities|Time|GetWorldDeltaSeconds) (Variables|Default|GetTurret%20Turn%20Speed)) false false)
      (bind _root (Variables|Default|GetRoot)
        (:then
          (Transformation|SetRelativeRotation _root (Math|Interpolation|RInterpTo (Variables|/Script/Engine.SceneComponent|GetRelativeRotation (Variables|Default|GetRoot)) (Math|Conversions|RotationFromXVector (Math|Vector|Normalize (Variables|Default|GetRotationalVector))) (Utilities|Time|GetWorldDeltaSeconds) (Variables|Default|GetTankBaseRotationSpeed)) false false)
          (bind _base (Variables|Default|GetBase)
            (:then
              (Physics|AddForce _base (* (Variables|Default|GetMovementVector) 1e+02) "None" true)
              (bind _root_2 (Variables|Default|GetRoot)
                (:then
                  (Transformation|SetWorldLocation _root_2 (Transformation|GetWorldLocation (Variables|Default|GetBase)) false false)
                  (CallFunction|HandleSlopes))
                (:else)))
            (:else)))
        (:else)))
    (:else)))

(event EventIRightStickX
  (params (Axis :type Float%20%28single-precision%29))
  ;[1 1 1] Right Stick
  (if (!= (Math|Float|Absolute(Float) Axis) 0.0)
    (Variables|Default|SetTurretRotationalVector (Math|Vector|MakeVector (stale EventIRightStickY Axis) Axis 0.0))))

(event EventIRightStickY
  (params (Axis :type Float%20%28single-precision%29))
  ;[1 1 1] Right Stick
  (if (!= (Math|Float|Absolute(Float) Axis) 0.0)
    (Variables|Default|SetTurretRotationalVector (Math|Vector|MakeVector Axis (stale EventIRightStickX Axis) 0.0))))

(event EventIKillPlayer
  ;[0.1611 1 0.08185] Health and Damage
  (CallFunction|PawnDeath))

(event Game|Damage|EventAnyDamage
  (params (Damage :type Float%20%28single-precision%29) (DamageType :type Damage%20Type%20Object%20Reference) (InstigatedBy :type Controller%20Object%20Reference) (DamageCauser :type Actor%20Object%20Reference))
  (bind _returnvalue (Utilities|GetClass DamageType))
  ;[0.1611 1 0.08185] Health and Damage
  (if (not (== _returnvalue "/Game/Destructibles/Radial.Radial_C"))
    (if (== _returnvalue "/Engine/EngineDamageTypes/DmgTypeBP_Environmental.DmgTypeBP_Environmental_C")
      (CallFunction|PawnDeath)
      (elif (not (Variables|Default|GetInvincible?))
        (Variables|Default|SetLastAttackedBy (Pawn|GetControlledPawn InstigatedBy))
        (bind _output_get (Variables|Default|SetCurrentHealth (- (Variables|Default|GetCurrentHealth) Damage)))
        (if (<= _output_get 0.0)
          (CallFunction|PawnDeath))))))

(event EventBeginPlay
  ;[1 1 1] BeginPlay
  (bind _returnvalue (Game|SpawnActorfromClass (Variables|Default|GetturretClass) (Math|Conversions|ToTransform(Vector) (Transformation|GetWorldLocation (Variables|Default|GetTurretSpawn))) "Undefined" 0 0))
  (Default|Init _returnvalue self)
  (Variables|Default|SetTurret _returnvalue))

(event EventLLeftTrigger
  (params (axis :type Float%20%28single-precision%29))
  ;[1 1 1] Throttle
  (Variables|Default|SetMovementVector (* (Transformation|GetActorForwardVector) (* (Math|Float|Clamp(Float) axis) (Variables|Default|GetTankSpeed)))))

(event EventILeftStickX
  (params (Axis :type Float%20%28single-precision%29))
  ;[1 1 1] Left Stick
  (if (!= (Math|Float|Absolute(Float) Axis) 0.0)
    (Variables|Default|SetRotationalVector (Math|Vector|MakeVector (stale EventILeftStickY Axis) Axis 0.0))))

(event EventIWeaponFire
  ;[0.1611 1 0.08185] Weapon fire
  (if (not (Variables|Default|GetWeaponFireCooldown))
    (CallFunction|WeaponFire)
    (bind _returnvalue (Utilities|Time|SetTimerbyEvent (delegate Custom|WeaponFire) (Variables|Default|GetFireDelay) true))))

(event EventIWeaponReleased
  ;[0.1611 1 0.08185] Weapon fire
  (Utilities|Time|ClearandInvalidateTimerbyHandle (stale EventIWeaponFire _returnvalue)))

(event Input|ActionEvents|InputActionDamageSelf
  (params (Key :type Key%20Structure))
  (bind _self self)
  (:Pressed
    (Game|Damage|ApplyDamage _self 25.0 (Pawn|GetController _self) 0 "/Script/Engine.DamageType")))

(event Input|KeyboardEvents|NumPadZero
  (params (Key :type Key%20Structure))
  (:Pressed
    (Game|Damage|ApplyDamage self 5e+01 0 0 "/Script/Engine.DamageType")))

(fn ConstructionScript)

(fn GetBase
  (return (Variables|Default|GetBase)))