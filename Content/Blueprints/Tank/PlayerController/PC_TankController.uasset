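; Player controller for a tank game that relays input to the controlled pawn and handles the player's death and respawn.
; Movement, turret, trigger, weapon fire and Tan-Kyo drift inputs are forwarded as interface messages.
; On a kill by another tank controller in DeathMatchGameMode, score interface actors credit the killer's team.
; Death destroys the pawn, notifies the game mode and starts a respawn timer using the game mode's delay.
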(event Custom|Killed
  (params (KilledBy :type Controller%20Object%20Reference))
  (bind _returnvalue (Game|GetGameMode))
  (Variables|Default|SetDead true)
  (bind _aspc_tank_controller (Utilities|Casting|CastToPC_TankController KilledBy)
    (:then
      (bind _asdeath_match_game_mode (Utilities|Casting|CastToDeathMatchGameMode (Game|GetGameMode))
        (:then
          (bind _outactors (Actor|GetAllActorswithInterface "/Game/CustomScripts/Interfaces/I_Score.I_Score_C"))
          (for _array_element _outactors
            (Class|IScore|AddScore(Message) _array_element (.playerteam (Variables|PC_TankController_C|GetPlayerInfo _aspc_tank_controller)) 1)
            (Actor|DestroyActor (Pawn|GetControlledPawn))
            (Class|IGamemode|PlayerKilled(Message) _returnvalue self)
            (bind _respawntime (Class|IGamemode|GetRespawnTime(Message) _returnvalue))
            (Utilities|Time|SetTimerbyEvent (delegate Custom|Respawn) _respawntime))
          (Development|PrintString "score added"))
        (:CastFailed
          (Actor|DestroyActor (Pawn|GetControlledPawn) :!label _label)
          (Class|IGamemode|PlayerKilled(Message) _returnvalue self)
          (bind _respawntime_2 (Class|IGamemode|GetRespawnTime(Message) _returnvalue))
          (Utilities|Time|SetTimerbyEvent (delegate Custom|Respawn) _respawntime_2))))
    (:CastFailed
      (goto _label))))

(event Custom|Respawn
  (Class|IGamemode|RespawnPlayer(Message) (Game|GetGameMode) self)
  (Variables|Default|SetDead false))

(event EventSetPlayerInfo
  (params (playerInfo :type Player%20Info%20Structure))
  (Variables|Default|SetPlayerInfo playerInfo))

(event Input|ActionEvents|InputActionWeaponFire
  (params (Key :type Key%20Structure))
  (bind _returnvalue (Pawn|GetControlledPawn))
  ;[0.1611 1 0.08185] Weapon fire
  (:Pressed
    (Class|ICharacterInterface|IWeaponFire(Message) _returnvalue))
  (:Released
    (Class|ICharacterInterface|IWeaponReleased(Message) _returnvalue)))

(event Input|ActionEvents|InputActionTan-KyoDrift
  (params (Key :type Key%20Structure))
  (bind _returnvalue (Pawn|GetControlledPawn))
  ;[0.1611 1 0.08185] Tan-Kyo Drift
  (:Pressed
    (Class|ICharacterInterface|ITan-Kyo-DriftEnabled(Message) _returnvalue))
  (:Released
    (Class|ICharacterInterface|ITan-Kyo-DriftDisabled(Message) _returnvalue)))

(event Input|AxisEvents|InputAxisLeftStickX
  (params (AxisValue :type Float%20%28single-precision%29))
  ;[0.1611 1 0.08185] Tank movement
  (Class|ICharacterInterface|ILeftStickX(Message) (Pawn|GetControlledPawn) AxisValue))

(event Input|AxisEvents|InputAxisLeftStickY
  (params (AxisValue :type Float%20%28single-precision%29))
  ;[0.1611 1 0.08185] Tank movement
  (Class|ICharacterInterface|ILeftStickY(Message) (Pawn|GetControlledPawn) AxisValue))

(event Input|AxisEvents|InputAxisRightStickX
  (params (AxisValue :type Float%20%28single-precision%29))
  ;[0.1611 1 0.08185] Turret movement
  (Class|ICharacterInterface|IRightStickX(Message) (Pawn|GetControlledPawn) AxisValue))

(event Input|AxisEvents|InputAxisRightStickY
  (params (AxisValue :type Float%20%28single-precision%29))
  ;[0.1611 1 0.08185] Turret movement
  (Class|ICharacterInterface|IRightStickY(Message) (Pawn|GetControlledPawn) AxisValue))

(event Input|AxisEvents|InputAxisLeftTrigger
  (params (AxisValue :type Float%20%28single-precision%29))
  (Class|ICharacterInterface|LLeftTrigger(Message) (Pawn|GetControlledPawn) AxisValue))

(fn ConstructionScript)