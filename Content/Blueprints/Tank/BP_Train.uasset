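; BP_Train is a train actor that repeatedly travels the length of a referenced track's spline.
; After a sync offset at BeginPlay, a timeline scaled to the movement duration lerps spline distance to set location and rotation, restarting after a delay.
; A Forward flag fixes the direction, with reverse runs playing the timeline backwards and adding 180 degrees of yaw.
; The construction script applies the configurable mesh and material.
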(event Custom|TrainMoves
  (bind _trackref (Variables|Default|GetTrackRef))
  (bind _trainmove (Variables|Default|GetTrainMove))
  (bind _track (Variables|/Game/Blueprints/Tank/BP_TrainTrack.BP_TrainTrack_C|GetTrack _trackref))
  (Components|Timeline|SetPlayRate _trainmove (/ 1.0 (Variables|Default|GetMovementDuration)))
  (if (Variables|Default|GetForward)
    (Components|Timeline|SetNewTime _trainmove 0.0)
    (bind _alpha (Timeline|TrainMove Play)
      (:Update
        (Variables|Default|SetAlpha _alpha)
        (if (Variables|Default|GetForward)
          (Transformation|SetActorLocationAndRotation (Spline|GetLocationatDistanceAlongSpline _track (Math|Float|Lerp 0.0 (Spline|GetSplineLength _track) (Variables|Default|GetAlpha)) "World") (Spline|GetRotationatDistanceAlongSpline _track (Math|Float|Lerp 0.0 (Spline|GetSplineLength _track) (Variables|Default|GetAlpha)) "Local"))
          (else
            (Transformation|SetActorLocationAndRotation (Spline|GetLocationatDistanceAlongSpline _track (Math|Float|Lerp 0.0 (Spline|GetSplineLength _track) (Variables|Default|GetAlpha)) "World") (Math|Rotator|MakeRotator (.Roll (Math|Rotator|BreakRotator (Spline|GetRotationatDistanceAlongSpline _track (Math|Float|Lerp 0.0 (Spline|GetSplineLength _track) (Variables|Default|GetAlpha)) "Local"))) (.Pitch (Math|Rotator|BreakRotator (Spline|GetRotationatDistanceAlongSpline _track (Math|Float|Lerp 0.0 (Spline|GetSplineLength _track) (Variables|Default|GetAlpha)) "Local"))) (+ (.Yaw (Math|Rotator|BreakRotator (Spline|GetRotationatDistanceAlongSpline _track (Math|Float|Lerp 0.0 (Spline|GetSplineLength _track) (Variables|Default|GetAlpha)) "Local"))) 1.8e+02))))))
      (:Finished
        (Utilities|FlowControl|Delay (Variables|Default|GetTrainDelay))
        (CallFunction|TrainMoves)))
    (else
      (Components|Timeline|SetNewTime _trainmove 1.0)
      (Timeline|TrainMove Reverse))))

(event EventBeginPlay
  (Utilities|FlowControl|Delay (Variables|Default|GetSyncOffset))
  (CallFunction|TrainMoves))

(event Collision|EventActorBeginOverlap
  (params (OtherActor :type Actor%20Object%20Reference)))

(event EventTick
  (params (DeltaSeconds :type Float%20%28single-precision%29)))

(fn ConstructionScript
  (bind _trainmesh (Variables|Default|GetTrainMesh))
  (Components|StaticMesh|SetStaticMesh _trainmesh (Variables|Default|GetTrainModel))
  (Rendering|Material|SetMaterial _trainmesh 0 (Variables|Default|GetModelMaterial)))