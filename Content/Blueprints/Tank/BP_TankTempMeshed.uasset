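; Twin-stick tank pawn that moves, drifts, fires projectiles and takes damage, driven mostly by interface input events.
; Left stick feeds FloatingPawnMovement and turns the base toward velocity, while right stick interpolates the turret's rotation.
; Tan-Kyo Drift adds clamped velocity-based impulses and quicker base turning.
; Held fire repeats on a timer with a cooldown; roll checks zero velocity, and depleted health destroys the actor.
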(event Custom|WeaponFire
  ;[0.1611 1 0.08185] Weapon fire
  (Game|SpawnActorfromClass "/Game/Blueprints/Tank/Projectiles/BP_SimpleProjectile.BP_SimpleProjectile_C" (Transformation|GetWorldTransform (Variables|Default|GetFirePoint)) "Undefined" 0 0)
  (Variables|Default|SetWeaponFireCooldown true)
  (Utilities|Time|SetTimerbyEvent (delegate Custom|ResetFire) (Variables|Default|GetFireDelay)))

(event Custom|ZeroVilocity
  ;[0.1611 1 0.08185] Fall rotation clamp
  (Variables|/Script/Engine.MovementComponent|SetVelocity (Variables|Default|GetFloatingPawnMovement) "0, 0, 0"))

(event Custom|ResetFire
  ;[0.1611 1 0.08185] Weapon fire
  (Variables|Default|SetWeaponFireCooldown false))

(event Custom|Tan-kyo-drift%20Ability
  ;[1 0.545 0] Tan-Kyo-Drift
  (CallFunction|DriftDisabled))

(event Custom|DriftReset
  ;[1 0.545 0] Tan-Kyo-Drift
  (Utilities|FlowControl|DoOnce false) ; enters at Reset
)

(event Custom|PawnDeath
  ;[0.1611 1 0.08185] Health and Damage
  (Actor|DestroyActor))

(event Custom|AddHealth
  (params (Amount :type Float%20%28single-precision%29))
  ;[0.1611 1 0.08185] Health and Damage
  (Variables|Default|SetCurrentHealth (Math|Float|Clamp(Float) (+ Amount (Variables|Default|GetCurrentHealth)) 0.0 (Variables|Default|GetMaxHealth))))

(event Custom|DriftDisabled
  ;[1 0.545 0] Tan-Kyo-Drift
  (Variables|Default|SetDriftActive false)
  (Variables|Default|SetTankBaseRotationSpeed 1.5)
  (CallFunction|DriftReset))

(event EventILeftStickX
  (params (Axis :type Float%20%28single-precision%29))
  (bind _floatingpawnmovement (Variables|Default|GetFloatingPawnMovement))
  (bind _tank_speed (Variables|Default|GetTank%20Speed))
  (bind _base (Variables|Default|GetBase))
  (bind _velocity (Variables|/Script/Engine.MovementComponent|GetVelocity _floatingpawnmovement))
  ;[1 0.545 0] Movement + Tan-Kyo Drift (Look into improving impulse and control)
  (Class|PawnMovementComponent|AddInputVector _floatingpawnmovement (Math|Vector|MakeVector (* (stale EventILeftStickY Axis) _tank_speed) (* Axis _tank_speed) 0.0) false)
  (if (Variables|Default|GetDriftActive)
    (Physics|AddImpulse (Variables|Default|GetBase) (Math|Vector|ClampVectorSize (* _velocity (Variables|Default|GetDriftImpulse)) 0.0 1.2e+03) "None" false))
  (if (> (Math|Vector|VectorLength _velocity) 0.0)
    (Transformation|SetRelativeRotation _base (Math|Interpolation|RInterpTo (Variables|/Script/Engine.SceneComponent|GetRelativeRotation _base) (Math|Conversions|RotationFromXVector (Math|Vector|Normalize _velocity)) (Utilities|Time|GetWorldDeltaSeconds) (Variables|Default|GetTankBaseRotationSpeed)) false false)
    ;[0.1611 1 0.08185] Fall rotation clamp
    (if (> (.roll (Transformation|GetWorldRotation (Variables|Default|GetBase))) 1e+01)
      (CallFunction|ZeroVilocity))))

(event EventILeftStickY
  (params (Axis :type Float%20%28single-precision%29))
  (bind _floatingpawnmovement (Variables|Default|GetFloatingPawnMovement))
  (bind _tank_speed (Variables|Default|GetTank%20Speed))
  (bind _base (Variables|Default|GetBase))
  (bind _velocity (Variables|/Script/Engine.MovementComponent|GetVelocity _floatingpawnmovement))
  ;[1 0.545 0] Movement + Tan-Kyo Drift (Look into improving impulse and control)
  (Class|PawnMovementComponent|AddInputVector _floatingpawnmovement (Math|Vector|MakeVector (* Axis _tank_speed) (* (stale EventILeftStickX Axis) _tank_speed) 0.0) false)
  (if (Variables|Default|GetDriftActive)
    (Physics|AddImpulse (Variables|Default|GetBase) (Math|Vector|ClampVectorSize (* _velocity (Variables|Default|GetDriftImpulse)) 0.0 1.2e+03) "None" false))
  (if (> (Math|Vector|VectorLength _velocity) 0.0)
    (Transformation|SetRelativeRotation _base (Math|Interpolation|RInterpTo (Variables|/Script/Engine.SceneComponent|GetRelativeRotation _base) (Math|Conversions|RotationFromXVector (Math|Vector|Normalize _velocity)) (Utilities|Time|GetWorldDeltaSeconds) (Variables|Default|GetTankBaseRotationSpeed)) false false)
    ;[0.1611 1 0.08185] Fall rotation clamp
    (if (> (.roll (Transformation|GetWorldRotation (Variables|Default|GetBase))) 1e+01)
      (CallFunction|ZeroVilocity))))

(event EventIRightStickX
  (params (Axis :type Float%20%28single-precision%29))
  ;[0.1611 1 0.08185] Turret rotation
  (if (> (Math|Vector|VectorLength (Math|Vector|MakeVector (* (stale EventIRightStickY Axis) -1.0) (* Axis 1.0) 0.0)) 0.25)
    (Variables|Default|SetDestrot (Math|Conversions|RotationFromXVector (Math|Vector|MakeVector (* (stale EventIRightStickY Axis) -1.0) (* Axis 1.0) 0.0)))
    (Transformation|SetWorldRotation (Variables|Default|GetSwivelyBit) (Math|Interpolation|RInterpTo (Transformation|GetWorldRotation (Variables|Default|GetSwivelyBit)) (Variables|Default|GetDestrot) (Utilities|Time|GetWorldDeltaSeconds) (Variables|Default|GetTurret%20Turn%20Speed)) false false)))

(event EventIRightStickY
  (params (Axis :type Float%20%28single-precision%29))
  ;[0.1611 1 0.08185] Turret rotation
  (if (> (Math|Vector|VectorLength (Math|Vector|MakeVector (* Axis -1.0) (* (stale EventIRightStickX Axis) 1.0) 0.0)) 0.25)
    (Variables|Default|SetDestrot (Math|Conversions|RotationFromXVector (Math|Vector|MakeVector (* Axis -1.0) (* (stale EventIRightStickX Axis) 1.0) 0.0)))
    (Transformation|SetWorldRotation (Variables|Default|GetSwivelyBit) (Math|Interpolation|RInterpTo (Transformation|GetWorldRotation (Variables|Default|GetSwivelyBit)) (Variables|Default|GetDestrot) (Utilities|Time|GetWorldDeltaSeconds) (Variables|Default|GetTurret%20Turn%20Speed)) false false)))

(event EventITan-Kyo-DriftEnabled
  ;[1 0.545 0] Tan-Kyo-Drift
  (Utilities|FlowControl|DoOnce false
    (:Completed
      (Variables|Default|SetDriftActive true)
      (Variables|Default|SetTankBaseRotationSpeed 2.5)
      (Utilities|Time|SetTimerbyEvent (delegate Custom|Tan-kyo-drift%20Ability) 0.0))))

(event EventITan-Kyo-DriftDisabled
  ;[1 0.545 0] Tan-Kyo-Drift
  (Variables|Default|SetDriftActive false)
  (Variables|Default|SetTankBaseRotationSpeed 1.5)
  (CallFunction|DriftReset))

(event Game|Damage|EventAnyDamage
  (params (Damage :type Float%20%28single-precision%29) (DamageType :type Damage%20Type%20Object%20Reference) (InstigatedBy :type Controller%20Object%20Reference) (DamageCauser :type Actor%20Object%20Reference))
  ;[0.1611 1 0.08185] Health and Damage
  (bind _output_get (Variables|Default|SetCurrentHealth (- (Variables|Default|GetCurrentHealth) Damage)))
  (if (<= _output_get 0.0)
    (CallFunction|PawnDeath)))

(event EventIWeaponFire
  ;[0.1611 1 0.08185] Weapon fire
  (Development|PrintString "fired")
  (if (not (Variables|Default|GetWeaponFireCooldown))
    (CallFunction|WeaponFire)
    (bind _returnvalue (Utilities|Time|SetTimerbyEvent (delegate Custom|WeaponFire) (Variables|Default|GetFireDelay) true))
    (else
      (Development|PrintString "cooldown active"))))

(event EventIWeaponReleased
  ;[0.1611 1 0.08185] Weapon fire
  (Development|PrintString "released")
  (Utilities|Time|ClearandInvalidateTimerbyHandle (stale EventIWeaponFire _returnvalue)))

(event Input|ActionEvents|InputActionReset
  (params (Key :type Key%20Structure))
  (bind _base (Variables|Default|GetBase))
  (bind _returnvalue (Transformation|GetWorldRotation _base))
  ;[1 0 0] Debug reset rotation
  (:Pressed
    (Variables|/Script/Engine.MovementComponent|SetVelocity (Variables|Default|GetFloatingPawnMovement) "0, 0, 0")
    (Transformation|SetWorldLocationAndRotation (Variables|Default|GetBase) (Transformation|GetWorldLocation _base) (Math|Rotator|MakeRotator 0.0 (.pitch _returnvalue) (.yaw _returnvalue)) false true)))

(fn ConstructionScript)