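; Tank mine projectile that drops behind its instigator and deals area damage when it explodes.
; On BeginPlay it teleports its Sphere 400 units behind the instigator.
; Both the hit check and the duration event trigger Explode, which sphere-traces PhysicsBody objects around the Cube within ExplosionDistance.
; Explode passes each hit actor to the parent's damage check, then destroys the mine; the trace's debug drawing is enabled.
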(event Custom|Explode
  (bind _cube (Variables|Default|GetCube))
  (bind _returnvalue (Transformation|GetWorldLocation _cube))
  (bind _outhits (Collision|MultiSphereTraceForObjects _returnvalue _returnvalue (Variables|Default|GetExplosionDistance) (Utilities|Array|MakeArray "ObjectTypeQuery4") false 0 "ForDuration"))
  (for _array_element _outhits
    (|CallParentFunction (.hitactor _array_element)))
  (Actor|DestroyActor))

(event EventBeginPlay
  (bind _returnvalue (Game|GetInstigator))
  (|CallParentFunction)
  (Transformation|SetWorldLocation (Variables|Default|GetSphere) (+ (Transformation|GetActorLocation _returnvalue) (* (Transformation|GetActorForwardVector _returnvalue) -4e+02)) false true))

(event Collision|EventActorBeginOverlap
  (params (OtherActor :type Actor%20Object%20Reference)))

(event EventTick
  (params (DeltaSeconds :type Float%20%28single-precision%29)))

(event EventCheckHitEnemyandDoDamage
  (params (DamagedActor :type Actor%20Object%20Reference))
  (CallFunction|Explode))

(event EventProjectileDuration
  (CallFunction|Explode)
  (|CallParentFunction))

(fn ConstructionScript
  (|CallParentFunction))