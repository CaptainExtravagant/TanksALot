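; Laser projectile for tanks, a child projectile Blueprint that behaves as a beam held on the firing tank's turret.
; On BeginPlay it caches the instigating tank and calls its LazorSloMo with the duration.
; Each tick it sweeps the Sphere to the turret fire point and matches its rotation plus an offset.
; Cube overlaps trigger the parent's hit-and-damage check, repeated every tick while the last overlapped actor stays inside.
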(event OnComponentBeginOverlap(Cube)
  (params (OverlappedComponent :type Primitive%20Component%20Object%20Reference) (OtherActor :type Actor%20Object%20Reference) (OtherComp :type Primitive%20Component%20Object%20Reference) (OtherBodyIndex :type Integer) (bFromSweep :type Boolean) (SweepResult :type Hit%20Result%20Structure%20%28by%20ref%29))
  (Variables|Default|SetCurrentOverllapingActor OtherActor)
  (CallFunction|CheckHitEnemyandDoDamage OtherActor))

(event EventBeginPlay
  (|CallParentFunction)
  (bind _tank (CallFunction|GetInstigatingTank))
  (bind _output_get (Variables|Default|SetInstigatingTank _tank))
  (Default|LazorSloMo _output_get (Variables|Default|GetDuration)))

(event Collision|EventActorBeginOverlap
  (params (OtherActor :type Actor%20Object%20Reference)))

(event EventTick
  (params (DeltaSeconds :type Float%20%28single-precision%29))
  (bind _sphere (Variables|Default|GetSphere)
    (:then
      (Transformation|SetWorldLocation _sphere (Transformation|GetWorldLocation (Variables|/Game/Blueprints/Tank/BP_Turret.BP_Turret_C|GetFirePoint (Variables|/Game/Blueprints/Tank/BP_Tank.BP_Tank_C|GetTurret (Variables|Default|GetInstigatingTank)))) true false)
      (bind _sphere_2 (Variables|Default|GetSphere)
        (:then
          (Transformation|SetWorldRotation _sphere_2 (Math|Rotator|CombineRotators (Transformation|GetWorldRotation (Variables|/Game/Blueprints/Tank/BP_Turret.BP_Turret_C|GetFirePoint (Variables|/Game/Blueprints/Tank/BP_Tank.BP_Tank_C|GetTurret (Variables|Default|GetInstigatingTank)))) (Variables|Default|GetOffsetRotator)) false false)
          (bind _currentoverllapingactor (Variables|Default|GetCurrentOverllapingActor)
            (:then
              (if (Collision|IsOverlappingActor (Variables|Default|GetCube) _currentoverllapingactor :!class /Script/Engine.PrimitiveComponent)
                (CallFunction|CheckHitEnemyandDoDamage _currentoverllapingactor)))
            (:else)))
        (:else)))
    (:else)))

(event EventCheckHitEnemyandDoDamage
  (params (DamagedActor :type Actor%20Object%20Reference))
  (|CallParentFunction DamagedActor))

(fn ConstructionScript
  (|CallParentFunction))