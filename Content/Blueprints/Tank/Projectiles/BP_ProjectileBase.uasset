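; BP_ProjectileBase is the base tank projectile, which deals damage on hit and destroys itself when its Duration timer expires.
; On BeginPlay it caches the team from the instigator's PC_TankController.
; A hit applies direct damage only to player-controlled BP_Tanks on another team, plus radial damage with no team check.
; GetInstigatingTank returns the firing tank, logging a failed cast.
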(event Custom|ProjectileDuration
  ;[0.1611 1 0.08185] Projectile Duration
  (Actor|DestroyActor))

(event Collision|EventHit
  (params (MyComp :type Primitive%20Component%20Object%20Reference) (Other :type Actor%20Object%20Reference) (OtherComp :type Primitive%20Component%20Object%20Reference) (bSelfMoved :type Boolean) (HitLocation :type Vector :default "0, 0, 0") (HitNormal :type Vector :default "0, 0, 0") (NormalImpulse :type Vector :default "0, 0, 0") (Hit :type Hit%20Result%20Structure%20%28by%20ref%29))
  ;[0.1611 1 0.08185] Hit Event
  (CallFunction|CheckHitEnemyandDoDamage Other)
  (Game|Damage|ApplyRadialDamage (Variables|Default|GetProjDam) HitLocation 5e+02 "/Game/Destructibles/Radial.Radial_C" 0 0 0 false "ECC_Pawn"))

(event EventBeginPlay
  ;[0.1611 1 0.08185] Projectile Duration
  (Utilities|Time|SetTimerbyEvent (delegate Custom|ProjectileDuration) (Variables|Default|GetDuration))
  ;[0.3382 1 0] Setting team number
  (bind _aspc_tank_controller (Utilities|Casting|CastToPC_TankController (Pawn|GetController (Game|GetInstigator))))
  (Variables|Default|SetTeam (.playerteam (Variables|/Game/Blueprints/Tank/PlayerController/PC_TankController.PC_TankController_C|GetPlayerInfo _aspc_tank_controller))))

(fn ConstructionScript)

(fn CheckHitEnemyandDoDamage
  (params (DamagedActor :type Actor%20Object%20Reference))
  (bind _asbp_tank (Utilities|Casting|CastToBP_Tank DamagedActor))
  (bind _aspc_tank_controller (Utilities|Casting|CastToPC_TankController (Pawn|GetController _asbp_tank)))
  (if (!= (.playerteam (Variables|/Game/Blueprints/Tank/PlayerController/PC_TankController.PC_TankController_C|GetPlayerInfo _aspc_tank_controller)) (Variables|Default|GetTeam))
    (Game|Damage|ApplyDamage DamagedActor (Variables|Default|GetProjDam) (Game|GetInstigatorController) 0 "/Script/Engine.DamageType")))

(fn GetInstigatingTank
  (bind _asbp_tank (Utilities|Casting|CastToBP_Tank (Game|GetInstigator))
    (:then
      (return _asbp_tank))
    (:CastFailed
      (Development|PrintString "cast to tank failed for projectile"))))