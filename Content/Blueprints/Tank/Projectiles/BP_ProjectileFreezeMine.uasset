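; Freeze mine projectile for tanks that temporarily takes away a player's control.
; On BeginPlay it teleports its Sphere component to a fixed distance behind the instigator.
; When a tank with a PC_TankController overlaps it, it disables that player's input, waits two seconds, restores input and destroys itself.
; BeginPlay and overlap both run the parent class logic first.
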(event EventBeginPlay
  (bind _returnvalue (Game|GetInstigator))
  (|CallParentFunction)
  (Transformation|SetWorldLocation (Variables|Default|GetSphere) (+ (Transformation|GetActorLocation _returnvalue) (* (Transformation|GetActorForwardVector _returnvalue) -4e+02)) false true))

(event Collision|EventActorBeginOverlap
  (params (OtherActor :type Actor%20Object%20Reference))
  (|CallParentFunction OtherActor)
  (bind _asbp_tank (Utilities|Casting|CastToBP_Tank OtherActor))
  (bind _aspc_tank_controller (Utilities|Casting|CastToPC_TankController (Pawn|GetController _asbp_tank)))
  (Default|DisablePlayerInput _aspc_tank_controller)
  (Utilities|FlowControl|Delay 2.0)
  (Default|EnablePlayerInput _aspc_tank_controller)
  (Actor|DestroyActor))

(fn ConstructionScript
  (|CallParentFunction))