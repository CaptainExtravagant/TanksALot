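; BP_SimpleProjectileBase is a base tank projectile that damages what it hits and expires after a set duration.
; On BeginPlay it starts a timer that destroys the actor, then copies the team from the instigator's PC_TankController player info.
; Hit events apply damage to any actor except the instigator.
; The stored team is not checked before damage, and a hit does not destroy the projectile here.
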(event Custom|ProjectileDuration
  ;[0.1611 1 0.08185] Projectile Duration
  (Actor|DestroyActor))

(event Collision|EventHit
  (params (MyComp :type Primitive%20Component%20Object%20Reference) (Other :type Actor%20Object%20Reference) (OtherComp :type Primitive%20Component%20Object%20Reference) (bSelfMoved :type Boolean) (HitLocation :type Vector :default "0, 0, 0") (HitNormal :type Vector :default "0, 0, 0") (NormalImpulse :type Vector :default "0, 0, 0") (Hit :type Hit%20Result%20Structure%20%28by%20ref%29))
  ;[0.1611 1 0.08185] Hit Event
  (CallFunction|CheckHitEnemyandDoDamage Other))

(event EventBeginPlay
  ;[0.1611 1 0.08185] Projectile Duration
  (Utilities|Time|SetTimerbyEvent (delegate Custom|ProjectileDuration) (Variables|Default|GetDurtation))
  (bind _aspc_tank_controller (Utilities|Casting|CastToPC_TankController (Pawn|GetController (Game|GetInstigator))))
  (Variables|Default|SetTeam (.playerteam (Variables|/Game/Blueprints/Tank/PlayerController/PC_TankController.PC_TankController_C|GetPlayerInfo _aspc_tank_controller))))

(fn ConstructionScript)

(fn CheckHitEnemyandDoDamage
  (params (DamagedActor :type Actor%20Object%20Reference))
  (if (not (== DamagedActor (Game|GetInstigator)))
    (Game|Damage|ApplyDamage DamagedActor (Variables|Default|GetProjDam) 0 0 "/Script/Engine.DamageType")))