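; BP_SimpleProjectileHoming is a tank projectile that steers toward enemy tanks and destroys itself after the parent's hit-and-damage check.
; On BeginPlay it ignores its instigator and searches immediately, with an optionally looping timer for further searches.
; Each search sphere-traces forward, sets an opposing-team, controller-possessed tank's Base as the ProjectileMovement homing target, then pauses the timer.
; Older distance-based targeting remains as disconnected nodes.
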(event Custom|LookForEnemies
  (bind _sphere (Variables|Default|GetSphere))
  (bind _returnvalue (Transformation|GetWorldLocation _sphere))
  (bind _outhits (Collision|MultiSphereTraceForObjects _returnvalue (+ _returnvalue (* (Math|Vector|GetForwardVector _sphere) (Variables|Default|GetHomingDistance))) 1.2e+03 (Utilities|Array|MakeArray "ObjectTypeQuery4") false (Variables|Default|GetIgnoreTanks) "None"))
  (for _array_element _outhits
    (bind _asbp_tank (Utilities|Casting|CastToBP_Tank (.hitactor _array_element)))
    (bind _aspc_tank_controller (Utilities|Casting|CastToPC_TankController (Pawn|GetController _asbp_tank)))
    (if (!= (.playerteam (Variables|/Game/Blueprints/Tank/PlayerController/PC_TankController.PC_TankController_C|GetPlayerInfo _aspc_tank_controller)) (Variables|Default|GetTeam))
      (Variables|/Script/Engine.ProjectileMovementComponent|SetHomingTargetComponent (Variables|Default|GetProjectileMovement) (Variables|/Game/Blueprints/Tank/BP_Tank.BP_Tank_C|GetBase _asbp_tank))
      (Class|KismetSystemLibrary|PauseTimer 0 "LookForEnemies"))))

(event EventBeginPlay
  (|CallParentFunction)
  (Utilities|Array|Add (Variables|Default|GetIgnoreTanks) (Game|GetInstigator))
  (Utilities|Time|SetTimerbyEvent (delegate Custom|LookForEnemies) (Variables|Default|GetHomingLoopTimer) (Variables|Default|GetShouldLoop))
  (CallFunction|LookforEnemies))

(event EventTick
  (params (DeltaSeconds :type Float%20%28single-precision%29))
  (|CallParentFunction DeltaSeconds))

(event EventCheckHitEnemyandDoDamage
  (params (DamagedActor :type Actor%20Object%20Reference))
  (|CallParentFunction DamagedActor)
  (Actor|DestroyActor))

(fn ConstructionScript
  (|CallParentFunction))