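; BP_ProjectileSplitShot is a tank projectile that splits into a fan of other projectiles.
; SpawnSplitProjectiles takes a projectile class and loops over ProjectileCount, spawning copies with lateral offsets and angular spread around the Sphere's up vector, then destroys itself.
; It swaps a nested split shot for BP_ProjectileSimple and passes an OffsetRotator to spawned lasers (BP_ProjectileLazor).
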(event EventBeginPlay
  (|CallParentFunction))

(event EventSpawnSplitProjectiles
  (params (Projectile :type BP%20Projectile%20Base%20Class%20Reference))
  (bind _projectilecount (Variables|Default|GetProjectileCount))
  (bind _projectilecount_2 (Variables|Default|GetProjectileCount))
  (bind _projectilecount_3 (Variables|Default|GetProjectileCount))
  (bind _projectilecount_4 (Variables|Default|GetProjectileCount))
  (bind _count (Variables|Default|GetCount))
  (bind _sphere (Variables|Default|GetSphere))
  (bind _returnvalue (Math|Vector|GetUpVector _sphere))
  (bind _returnvalue_2 (/ _projectilecount_4 2))
  (bind _returnvalue_3 (/ _projectilecount_3 2))
  (bind _returnvalue_4 (- _count _projectilecount_2))
  (bind _returnvalue_5 (+ _projectilecount 1))
  (bind _returnvalue_6 (Math|Conversions|ToFloat(Integer) _returnvalue_2))
  (bind _returnvalue_7 (Math|Conversions|ToFloat(Integer) _returnvalue_4))
  (bind _returnvalue_8 (Math|Conversions|ToFloat(Integer) _returnvalue_3))
  (bind _returnvalue_9 (* _returnvalue_5 5.0))
  (bind _returnvalue_10 (+ _returnvalue_6 0.5))
  (bind _returnvalue_11 (+ _returnvalue_8 0.5))
  (bind _returnvalue_12 (* _returnvalue_10 _returnvalue_9))
  (bind _returnvalue_13 (* _returnvalue_11 1e+01))
  (bind _returnvalue_14 (* _returnvalue_13 _returnvalue_7))
  (bind _returnvalue_15 (+ _returnvalue_14 _returnvalue_12))
  (bind _returnvalue_16 (Math|Vector|RotatorfromAxisandAngle _returnvalue _returnvalue_15))
  (Variables|Default|SetProjectileType Projectile)
  (while (< (Variables|Default|GetCount) (Variables|Default|GetProjectileCount))
    (Utilities|IsValid (Game|GetInstigator)
      (:Is%20Valid
        (if (== (Variables|Default|GetProjectileType) "BP_ProjectileSplitShot_C")
          (Development|PrintString "Split shot not allowed, setting projectile type to simple")
          (Variables|Default|SetProjectileType "/Game/Blueprints/Tank/Projectiles/BP_ProjectileSimple.BP_ProjectileSimple_C")
          (else
            (Variables|Default|SetOffsetRotator _returnvalue_16)))
        (bind _returnvalue_17 (Game|SpawnActorfromClass (Variables|Default|GetProjectileType) (Math|Transform|MakeTransform (+ (Transformation|GetActorLocation) (- (* (Transformation|GetActorRightVector) (* (Variables|Default|GetCount) (Variables|Default|GetLateralOffset))) (* (Transformation|GetActorRightVector) (* (- (Variables|Default|GetProjectileCount) (Variables|Default|GetCount)) (/ (Variables|Default|GetLateralOffset) 2.0))))) (Math|Rotator|CombineRotators (Transformation|GetActorRotation) _returnvalue_16) "1,1,1") "AdjustIfPossibleButDontSpawnIfColliding" 0 (Game|GetInstigator)))
        (bind _asbp_projectile_lazor (Utilities|Casting|CastToBP_ProjectileLazor _returnvalue_17)
          (:then
            (Variables|/Game/Blueprints/Tank/Projectiles/BP_ProjectileLazor.BP_ProjectileLazor_C|SetOffsetRotator _asbp_projectile_lazor (Variables|Default|GetOffsetRotator)))
          (:CastFailed
            _))
        (Math|Integer|IncrementInt (Variables|Default|GetCount)))
      (:Is%20Not%20Valid
        (Development|PrintString "not valid"))))
  (Actor|DestroyActor))

(fn ConstructionScript
  (|CallParentFunction))