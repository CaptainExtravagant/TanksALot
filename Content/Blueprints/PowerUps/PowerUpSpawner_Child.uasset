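; Child power-up spawner that grants a speed, damage, shield or split-shot power-up to tanks that overlap it.
; On overlap, it sends the power-up type and effect time to any BP_Tank not already powered up.
; The construction script sets the text label from the type.
; A RandomisePickUp event, not called in this graph, re-rolls the type every second in a delay loop without updating the label.
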(event EventBeginPlay
  (|CallParentFunction) ; This node is disabled and will not be called.\nDrag off pins to build functionality.
)

(event Collision|EventActorBeginOverlap
  (params (OtherActor :type Actor%20Object%20Reference))
  (|CallParentFunction OtherActor)
  (bind _asbp_tank (Utilities|Casting|CastToBP_Tank OtherActor))
  (Variables|Default|SetTank _asbp_tank)
  (if (not (Variables|/Game/Blueprints/Tank/BP_Tank.BP_Tank_C|GetPoweredUp? _asbp_tank))
    (Class|IPowerUpPickedUp|PowerUpPickedUp(Message) _asbp_tank (Variables|Default|GetPowerUpType) (Variables|Default|GetEffectTime))))

(event EventTick
  (params (DeltaSeconds :type Float%20%28single-precision%29))
  (|CallParentFunction DeltaSeconds) ; This node is disabled and will not be called.\nDrag off pins to build functionality.
)

(event EventRandomisePickUp
  ;[1 1 1] Random?
  (Variables|Default|SetPowerUpType (Utilities|Select :Index (Math|Random|RandomInteger (- (|GetNumEnumEntries) 1)) :Option%200 "NewEnumerator0" :Option%201 "NewEnumerator1" :Option%202 "NewEnumerator2" :Option%203 "NewEnumerator3") :!label _label)
  (Utilities|FlowControl|Delay 1.0)
  (goto _label))

(fn ConstructionScript
  (|CallParentFunction)
  (switch Utilities|FlowControl|Switch|SwitchonPowerUpEnum (Variables|Default|GetPowerUpType)
    (:NewEnumerator0
      (Variables|Default|SetPowerUpName "Speed"))
    (:NewEnumerator1
      (Variables|Default|SetPowerUpName "Damage"))
    (:NewEnumerator2
      (Variables|Default|SetPowerUpName "Shield"))
    (:NewEnumerator3
      (Variables|Default|SetPowerUpName "SplitShot")))
  (Rendering|Components|TextRender|SetText (Variables|Default|GetTextRender) (Variables|Default|GetPowerUpName)))