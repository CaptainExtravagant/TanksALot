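; Power-up pickup that gives a tank a different projectile type for a limited time when the tank overlaps it.
; On begin play it replaces the effect time with its default overwrite value, then on overlap passes the projectile class and that time to BP_Tank.
; The construction script labels the pickup's text render with the projectile class's display name, and all active handlers call their parent versions first.
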(event EventBeginPlay
  (|CallParentFunction)
  (Variables|Default|SetEffectTime (Variables|Default|GetEffectTimeDefaultOverwrite)))

(event Collision|EventActorBeginOverlap
  (params (OtherActor :type Actor%20Object%20Reference))
  (|CallParentFunction OtherActor)
  (bind _asbp_tank (Utilities|Casting|CastToBP_Tank OtherActor))
  (bind _output_get (Variables|Default|SetTank _asbp_tank))
  (Default|SetProjectileType _output_get (Variables|Default|GetProjectileType) (Variables|Default|GetEffectTime)))

(event EventTick
  (params (DeltaSeconds :type Float%20%28single-precision%29)))

(fn ConstructionScript
  (|CallParentFunction)
  (Rendering|Components|TextRender|SetText (Variables|Default|GetTextRender) (Utilities|Text|ToText(String) (Utilities|GetClassDisplayName (Variables|Default|GetProjectileType)))))