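; BP_Tank is a twin-stick tank pawn with timed power-ups.
; The left stick drives FloatingPawnMovement and eases the base toward its velocity, while the right stick swivels the turret at constant speed beyond a deadzone.
; Power-up pickups temporarily multiply max speed or set invincibility, reverting after a delay.
; Pressing fire spawns one actor at the fire point, currently a CameraActor rather than a projectile.
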(event Custom|SpeedPowerUp
  ;[1 1 1] Speed PowerUp
  (Variables|/Script/Engine.FloatingPawnMovement|SetMaxSpeed (Variables|Default|GetFloatingPawnMovement) (* (Variables|Default|GetDefaultTankSpeed) 1e+02))
  (Utilities|FlowControl|Delay (Variables|PowerUp|GetPowerUpTimer))
  (Variables|/Script/Engine.FloatingPawnMovement|SetMaxSpeed (Variables|Default|GetFloatingPawnMovement) (Variables|Default|GetDefaultTankSpeed))
  (Development|PrintString "Speed Boost Over"))

(event Custom|ShieldPowerUp
  ;[1 1 1] Shield PowerUp
  (Variables|Default|SetInvincible? true)
  (Utilities|FlowControl|Delay (Variables|PowerUp|GetPowerUpTimer))
  (Variables|Default|SetInvincible? false)
  (Development|PrintString "Invincibility Over"))

(event EventPowerUpPickedUp
  (params (PowerUpType :type PowerUpEnum%20Enum :default "NewEnumerator0") (PowerUpActiveTimer :type Float%20%28single-precision%29))
  ;[1 1 1] PowerUps
  (Variables|PowerUp|SetPowerUpTimer PowerUpActiveTimer)
  (switch Utilities|FlowControl|Switch|SwitchonPowerUpEnum PowerUpType
    (:NewEnumerator0
      (CallFunction|SpeedPowerUp))
    (:NewEnumerator2
      (CallFunction|ShieldPowerUp))))

(event Input|ActionEvents|InputActionWeaponFire
  (params (Key :type Key%20Structure))
  ;[1 0.545 0] Basic weapon fire (Needs to be hold to fire)
  (:Pressed
    (Game|SpawnActorfromClass "/Script/Engine.CameraActor" (Transformation|GetWorldTransform (Variables|Default|GetFirePoint)) "Undefined" 0 0)))

(event Input|AxisEvents|InputAxisLeftStickX
  (params (AxisValue :type Float%20%28single-precision%29))
  (bind _floatingpawnmovement (Variables|Default|GetFloatingPawnMovement))
  (bind _base (Variables|Default|GetBase))
  (bind _tank_speed (Variables|Default|GetTank%20Speed))
  (bind _velocity (Variables|/Script/Engine.MovementComponent|GetVelocity _floatingpawnmovement))
  ;[1 0.545 0] Movement (Refine the movement)
  (Class|PawnMovementComponent|AddInputVector _floatingpawnmovement (Math|Vector|MakeVector (* (stale Input|AxisEvents|InputAxisLeftStickY AxisValue) _tank_speed) (* AxisValue _tank_speed) 0.0) false)
  (if (> (Math|Vector|VectorLength _velocity) 0.0)
    (Transformation|SetRelativeRotation _base (Math|Interpolation|RInterpTo (Variables|/Script/Engine.SceneComponent|GetRelativeRotation _base) (Math|Conversions|RotationFromXVector (Math|Vector|Normalize _velocity)) (Utilities|Time|GetWorldDeltaSeconds) (Variables|Default|GetTankBaseRotationSpeed)) false false)))

(event Input|AxisEvents|InputAxisLeftStickY
  (params (AxisValue :type Float%20%28single-precision%29))
  (bind _floatingpawnmovement (Variables|Default|GetFloatingPawnMovement))
  (bind _base (Variables|Default|GetBase))
  (bind _tank_speed (Variables|Default|GetTank%20Speed))
  (bind _velocity (Variables|/Script/Engine.MovementComponent|GetVelocity _floatingpawnmovement))
  ;[1 0.545 0] Movement (Refine the movement)
  (Class|PawnMovementComponent|AddInputVector _floatingpawnmovement (Math|Vector|MakeVector (* AxisValue _tank_speed) (* (stale Input|AxisEvents|InputAxisLeftStickX AxisValue) _tank_speed) 0.0) false)
  (if (> (Math|Vector|VectorLength _velocity) 0.0)
    (Transformation|SetRelativeRotation _base (Math|Interpolation|RInterpTo (Variables|/Script/Engine.SceneComponent|GetRelativeRotation _base) (Math|Conversions|RotationFromXVector (Math|Vector|Normalize _velocity)) (Utilities|Time|GetWorldDeltaSeconds) (Variables|Default|GetTankBaseRotationSpeed)) false false)))

(event Input|AxisEvents|InputAxisRightStickX
  (params (AxisValue :type Float%20%28single-precision%29))
  (if (> (Math|Vector|VectorLength (Math|Vector|MakeVector (* AxisValue -1.0) (* (stale Input|AxisEvents|InputAxisRightStickY AxisValue) -1.0) 0.0)) 0.25)
    (Variables|Default|SetDestrot (Math|Conversions|RotationFromXVector (Math|Vector|MakeVector (* AxisValue -1.0) (* (stale Input|AxisEvents|InputAxisRightStickY AxisValue) -1.0) 0.0)))
    (Transformation|SetWorldRotation (Variables|Default|GetSwivelyBit) (Class|KismetMathLibrary|RInterptoConstant (Transformation|GetWorldRotation (Variables|Default|GetSwivelyBit)) (Variables|Default|GetDestrot) (Utilities|Time|GetWorldDeltaSeconds) (Variables|Default|GetTurret%20Turn%20Speed)) false false)))

(event Input|AxisEvents|InputAxisRightStickY
  (params (AxisValue :type Float%20%28single-precision%29))
  (if (> (Math|Vector|VectorLength (Math|Vector|MakeVector (* (stale Input|AxisEvents|InputAxisRightStickX AxisValue) -1.0) (* AxisValue -1.0) 0.0)) 0.25)
    (Variables|Default|SetDestrot (Math|Conversions|RotationFromXVector (Math|Vector|MakeVector (* (stale Input|AxisEvents|InputAxisRightStickX AxisValue) -1.0) (* AxisValue -1.0) 0.0)))
    (Transformation|SetWorldRotation (Variables|Default|GetSwivelyBit) (Class|KismetMathLibrary|RInterptoConstant (Transformation|GetWorldRotation (Variables|Default|GetSwivelyBit)) (Variables|Default|GetDestrot) (Utilities|Time|GetWorldDeltaSeconds) (Variables|Default|GetTurret%20Turn%20Speed)) false false)))

(fn ConstructionScript
  (Variables|/Script/Engine.FloatingPawnMovement|SetMaxSpeed (Variables|Default|GetFloatingPawnMovement) (Variables|Default|GetDefaultTankSpeed)))