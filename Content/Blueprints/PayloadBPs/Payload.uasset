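; Payload is the escort objective for the payload game mode, destroying itself in any map not running that mode.
; Init follows linked PayloadPathControlPoints actors from the beginning point to build the InterpToMovement path.
; Each tick it counts friendly and enemy tanks overlapping its sphere, enabling movement only with friendlies present and no enemies.
; Movement is paused by toggling the component's tick, and the cube rotates to face its velocity.
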(event Custom|Init
  (bind _outactors (Actor|GetAllActorsOfClass "/Game/Blueprints/PayloadBPs/PayloadPathControlPoints.PayloadPathControlPoints_C"))
  ;[1 1 1] Creates linked list of control points
  (bind _array_element (Utilities|Array|ForEachLoopwithBreak _outactors :!label _label)
    (:LoopBody
      (if (Variables|/Game/Blueprints/PayloadBPs/PayloadPathControlPoints.PayloadPathControlPoints_C|GetIsBeginning _array_element)
        (Variables|Default|SetStartPoint _array_element)
        (goto _label Break)))
    (:Completed
      (bind _output_get (Variables|Default|SetPoint (Variables|Default|GetStartPoint)))
      (Utilities|AddPointtoArray _output_get)
      (Variables|Default|SetPoint (Variables|/Game/Blueprints/PayloadBPs/PayloadPathControlPoints.PayloadPathControlPoints_C|GetNextControlPoint (Variables|Default|GetPoint)))
      (while (Utilities|IsValid (Variables|/Game/Blueprints/PayloadBPs/PayloadPathControlPoints.PayloadPathControlPoints_C|GetNextControlPoint (Variables|Default|GetPoint)))
        (Variables|Default|SetPoint (Variables|/Game/Blueprints/PayloadBPs/PayloadPathControlPoints.PayloadPathControlPoints_C|GetNextControlPoint (Variables|Default|GetPoint)))
        (Utilities|AddPointtoArray (Variables|Default|GetPoint)))
      (Variables|/Game/Blueprints/PayloadBPs/PayloadPathControlPoints.PayloadPathControlPoints_C|SetIsEnd (Variables|Default|GetPoint) true)
      (Class|InterptoMovementComponent|FinaliseControlPoints (Variables|Default|GetInterpToMovement)))))

(event EventBeginPlay
  ;[1 1 1] Check for correct game mode - allows this to be placed in any map
  (Utilities|Casting|CastToPayloadGameMode (Game|GetGameMode)
    (:then
      (Components|Tick|SetComponentTickEnabled (Variables|Default|GetInterpToMovement) false))
    (:CastFailed
      (Actor|DestroyActor))))

(event EventTick
  (params (DeltaSeconds :type Float%20%28single-precision%29))
  (bind _interptomovement (Variables|Default|GetInterpToMovement))
  (bind _velocity (Variables|/Script/Engine.MovementComponent|GetVelocity _interptomovement))
  (if (> (Math|Vector|VectorLength _velocity) 0.0)
    (Transformation|SetWorldRotation (Variables|Default|GetCube) (Math|Rotator|MakeRotfromX _velocity) false false))
  (bind _outactors (Actor|GetAllActorsOfClass "/Game/Blueprints/Tank/BP_Tank.BP_Tank_C"))
  (for _array_element _outactors
    (if (Collision|IsOverlappingActor (Variables|Default|GetSphere) _array_element :!class /Script/Engine.PrimitiveComponent)
      (Utilities|Array|AddUnique (Variables|Default|GetOverlappingTanks) _array_element)
      (else
        (Utilities|Array|RemoveItem (Variables|Default|GetOverlappingTanks) _array_element))))
  (for _array_element_2 (Variables|Default|GetOverlappingTanks)
    (Utilities|IsValid _array_element_2
      (:Is%20Valid
        (bind _aspc_tank_controller (Utilities|Casting|CastToPC_TankController (Pawn|GetController _array_element_2)))
        (Utilities|IsEnemy _aspc_tank_controller
          (:Friend
            (Math|Integer|IncrementInt (Variables|Default|GetOverlappingFriendlyCount)))
          (:Enemy
            (Math|Integer|IncrementInt (Variables|Default|GetOverlappingEnemyCount)))))
      (:Is%20Not%20Valid
        (Utilities|Array|RemoveItem (Variables|Default|GetOverlappingTanks) _array_element_2))))
  (if (> (Variables|Default|GetOverlappingEnemyCount) 0)
    (Components|Tick|SetComponentTickEnabled (Variables|Default|GetInterpToMovement) false :!label _label)
    (elif (> (Variables|Default|GetOverlappingFriendlyCount) 0)
      (Components|Tick|SetComponentTickEnabled (Variables|Default|GetInterpToMovement) true)
      (else
        (goto _label))))
  (Variables|Default|SetOverlappingEnemyCount 0)
  (Variables|Default|SetOverlappingFriendlyCount 0))

(fn ConstructionScript)