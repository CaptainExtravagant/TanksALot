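; Payload mode path control point actor that awards score when a payload reaches the end of the path.
; On BeginPlay it destroys itself outside PayloadGameMode, and enables its box's query collision only when flagged IsEnd.
; The end point caches the first valid I_Score actor as ScoreManager.
; An overlapping Payload makes it send that manager a fixed score for the payload's team and print a debug message.
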(event OnComponentBeginOverlap(Box)
  (params (OverlappedComponent :type Primitive%20Component%20Object%20Reference) (OtherActor :type Actor%20Object%20Reference) (OtherComp :type Primitive%20Component%20Object%20Reference) (OtherBodyIndex :type Integer) (bFromSweep :type Boolean) (SweepResult :type Hit%20Result%20Structure%20%28by%20ref%29))
  (bind _aspayload (Utilities|Casting|CastToPayload OtherActor))
  (Class|IScore|AddScore(Message) (Variables|Default|GetScoreManager) (Variables|/Game/Blueprints/PayloadBPs/Payload.Payload_C|GetTeam _aspayload) 10)
  (Development|PrintString "payload has reached the end"))

(event EventBeginPlay
  (Utilities|Casting|CastToPayloadGameMode (Game|GetGameMode)
    (:then
      (if (Variables|Default|GetIsEnd)
        (Collision|SetCollisionEnabled (Variables|Default|GetBox) "QueryOnly")
        (bind _outactors (Actor|GetAllActorswithInterface "/Game/CustomScripts/Interfaces/I_Score.I_Score_C"))
        (bind _array_element (Utilities|Array|ForEachLoopwithBreak _outactors :!label _label)
          (:LoopBody
            (Utilities|IsValid _array_element
              (:Is%20Valid
                (Variables|Default|SetScoreManager _array_element)
                (goto _label Break)))))
        (else
          (Collision|SetCollisionEnabled (Variables|Default|GetBox) "NoCollision"))))
    (:CastFailed
      (Actor|DestroyActor))))

(fn ConstructionScript)