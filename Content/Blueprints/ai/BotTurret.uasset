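; BotTurret is the turret actor for an AI-controlled tank, keeping itself mounted on the tank and aimed at that tank's current target.
; Each tick it moves itself to the world location of the tank's TurretSpawn component, following by position copy within this Blueprint.
; It then calls RotateToFaceTarget, which builds a rotation from the direction to CurrentTarget and applies it instantly, with no interpolation or validity check.
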(event EventBeginPlay)

(event Collision|EventActorBeginOverlap
  (params (OtherActor :type Actor%20Object%20Reference)))

(event EventTick
  (params (DeltaSeconds :type Float%20%28single-precision%29))
  (bind _tank (Variables|Default|GetTank))
  (bind _turretspawn (Variables|/Game/Blueprints/ai/DeathMatchBot.DeathMatchBot_C|GetTurretSpawn _tank))
  (bind _returnvalue (Transformation|GetWorldLocation _turretspawn))
  (Transformation|SetActorRelativeLocation (Math|Vector|MakeVector (.x _returnvalue) (.y _returnvalue) (.z _returnvalue)))
  (CallFunction|RotatetoFaceTarget))

(fn ConstructionScript)

(fn RotatetoFaceTarget
  (Transformation|SetActorRelativeRotation (Math|Conversions|RotationFromXVector (* (- (Transformation|GetActorLocation) (Transformation|GetActorLocation (Variables|/Game/Blueprints/ai/DeathMatchBot.DeathMatchBot_C|GetCurrentTarget (Variables|Default|GetTank)))) -1.0))))