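; AI tank bot that spawns its own turret and hunts a randomly chosen tank on an opposing team.
; Each tick it recomputes a navmesh path to the target, drawing debug spheres, and line-traces for visibility.
; It drives by adding force to its mesh along the path, firing timer-delayed projectiles when the visible target is within stopping distance.
; With line of sight, the body turns toward the target once its angle from the turret reaches the fire arc.
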(event Custom|WeaponFire
  (bind _turret (Variables|Default|GetTurret))
  (bind _firepoint (Variables|/Game/Blueprints/ai/tmpBotTurret.tmpBotTurret_C|GetFirePoint _turret))
  (bind _returnvalue (Transformation|GetWorldTransform _firepoint))
  (Game|SpawnActorfromClass (Variables|Default|GetProjectileType) (Math|Transform|MakeTransform (.location _returnvalue) (.rotation _returnvalue) "1,1,1") "Undefined" 0 self)
  (Variables|Default|SetWeaponCooldown true)
  (Utilities|Time|SetTimerbyEvent (delegate Custom|ResetFire) (Variables|Default|GetFireDelay)))

(event Custom|TargetDie
  (CallFunction|GetNewTarget))

(event Custom|ResetFire
  (Variables|Default|SetWeaponCooldown false))

(event EventTick
  (params (DeltaSeconds :type Float%20%28single-precision%29))
  (CallFunction|GetNewTarget)
  (CallFunction|GetPathtoTarget)
  (bind _lineofsight (CallFunction|LineOfSight))
  (if _lineofsight
    (CallFunction|ShouldtheBodyRotate)
    (if (>= (Variables|Default|GetDistanceTurned) (Variables|Default|GetFireArc))
      (CallFunction|RotatetoFaceTarget))
    (bind _distance (CallFunction|GetDistancetoCurrentTarget))
    (if (< _distance (Variables|Default|GetStoppingDistance))
      (Development|PrintString "FIRE")
      (if (not (Variables|Default|GetWeaponCooldown))
        (CallFunction|WeaponFire)
        (Utilities|Time|SetTimerbyEvent (delegate Custom|WeaponFire) (Variables|Default|GetFireDelay) true))
      (else
        (CallFunction|RotatetoFacePath)
        (Physics|AddForce (Variables|Default|GetStaticMesh) (* (Math|Vector|GetForwardVector (Variables|Default|GetStaticMesh)) (Variables|Default|GetSpeed)) "None" true)))
    (elif (> (Utilities|Array|Length (Variables|Default|GetPathToTarget)) 0)
      (CallFunction|RotatetoFacePath)
      (Physics|AddForce (Variables|Default|GetStaticMesh) (* (Math|Vector|GetForwardVector (Variables|Default|GetStaticMesh)) (Variables|Default|GetSpeed)) "None" true)
      (if (<= (Math|Vector|VectorLength (- (Transformation|GetActorLocation) (Utilities|Array|Get(acopy) (Variables|Default|GetPathToTarget) (Variables|Default|GetPathId)))) 5e+02)
        (bind _result (Math|Integer|IncrementInt (Variables|Default|GetPathId))
          (:%20%20
            (Variables|Default|SetPathId _result)
            (if (> (Variables|Default|GetPathId) (Utilities|Array|Length (Variables|Default|GetPathToTarget)))
              (Variables|Default|SetPathId 0))))))))

(event EventBeginPlay
  (CallFunction|GetNewTarget)
  (bind _returnvalue (Game|SpawnActorfromClass "/Game/Blueprints/ai/tmpBotTurret.tmpBotTurret_C" (Transformation|GetWorldTransform (Variables|Default|GetTurretSpawn)) "Undefined" 0 0))
  (bind _output_get (Variables|Default|SetTurret _returnvalue))
  (Variables|/Game/Blueprints/ai/tmpBotTurret.tmpBotTurret_C|SetTank _output_get self))

(fn ConstructionScript)

(fn GetDistancetoCurrentTarget
  (return (Math|Vector|VectorLength (- (Transformation|GetActorLocation (Variables|Default|GetCurrentTarget)) (Transformation|GetActorLocation)))))

(fn LineOfSight
  (bind _outhit (Collision|LineTraceByChannel (Transformation|GetActorLocation) (Transformation|GetActorLocation (Variables|Default|GetCurrentTarget)) "TraceTypeQuery1" false 0 "None"))
  (if (== (.HitActor (Collision|BreakHitResult _outhit)) (Variables|Default|GetCurrentTarget))
    (Variables|Default|SetLastKnownDirection (.Location (Collision|BreakHitResult _outhit))))
  (return (== (.HitActor (Collision|BreakHitResult _outhit)) (Variables|Default|GetCurrentTarget))))

(fn RotatetoFaceTarget
  (Transformation|SetActorRelativeRotation (Math|Rotator|FindLookatRotation (Transformation|GetActorLocation) (Transformation|GetActorLocation (Variables|Default|GetCurrentTarget)))))

(fn GetPathtoTarget
  (bind _outactors (Actor|GetAllActorsOfClass "/Script/NavigationSystem.NavMeshBoundsVolume"))
  (bind _returnvalue (Class|NavigationSystemV1|FindPathtoLocationSynchronously (Utilities|Array|Get(acopy) _outactors) (Transformation|GetActorLocation) (Transformation|GetActorLocation (Variables|Default|GetCurrentTarget)) 0 0))
  (bind _output_get (Variables|Default|SetPathToTarget (Variables|/Script/NavigationSystem.NavigationPath|GetPathPoints _returnvalue)))
  (Utilities|Array|RemoveIndex _output_get)
  (Variables|Default|SetPathId 0)
  (for _array_element _output_get
    (Rendering|Debug|DrawDebugSphere _array_element 5e+01 12 "(R=1.000000,G=0.000000,B=0.044905,A=1.000000)" 0.0 5e+01)))

(fn RotatetoFacePath
  (bind _pathtotarget (Variables|Default|GetPathToTarget))
  (bind _pathid (Variables|Default|GetPathId))
  (bind _output (Utilities|Array|Get(acopy) _pathtotarget _pathid))
  (if (> (Utilities|Array|Length _pathtotarget) 0)
    (Transformation|SetActorRelativeRotation (Math|Rotator|FindLookatRotation (Transformation|GetActorLocation) (Math|Vector|MakeVector (.x _output) (.y _output) (.z (Transformation|GetActorLocation)))))))

(fn RotateTurrettoFaceTarget
  (bind _turret (Variables|Default|GetTurret))
  (bind _returnvalue (Transformation|GetActorLocation _turret))
  (Transformation|SetActorRelativeRotation _turret (Math|Rotator|FindLookatRotation _returnvalue (- (Transformation|GetActorLocation (Variables|Default|GetCurrentTarget)) _returnvalue))))

(fn ShouldtheBodyRotate
  (Variables|Default|SetDistanceTurned (Class|KismetMathLibrary|DegAcos (Math|Vector|DotProduct (Transformation|GetActorForwardVector) (Math|Vector|GetForwardVector (Variables|/Game/Blueprints/ai/tmpBotTurret.tmpBotTurret_C|GetStaticMesh (Variables|Default|GetTurret)))))))

(fn GetNewTarget
  (if (== (Variables|Default|GetCurrentTarget) 0)
    (bind _outactors (Actor|GetAllActorsOfClass "/Game/Blueprints/Tank/BP_Tank.BP_Tank_C"))
    (Utilities|Array|Shuffle _outactors)
    (for _array_element _outactors
      (bind _aspc_tank_controller (Utilities|Casting|CastToPC_TankController (Pawn|GetController _array_element)))
      (if (!= (.playerteam (Variables|/Game/Blueprints/Tank/PlayerController/PC_TankController.PC_TankController_C|GetPlayerInfo _aspc_tank_controller)) (.playerteam (Variables|Default|GetTankInfo)))
        (bind _output_get (Variables|Default|SetCurrentTarget _array_element))
        (bind _asbp_tank (Utilities|Casting|CastToBP_Tank _output_get))
        (EventDispatchers|BindEventtoPlayerDied _asbp_tank (EventDispatchers|CreateEvent :!event Custom|TargetDie))))))