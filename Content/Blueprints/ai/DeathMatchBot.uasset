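; DeathMatchBot is an AI tank for deathmatch that spawns its own BotTurret and shows a team-coloured decal.
; It targets a random player or bot tank, switching to whoever damages it, and at zero health requests a respawn and scores for its last attacker's team.
; Each tick it recomputes a debug-drawn navmesh path, drives with physics force, and fires on a timer when a line trace confirms a target in range.
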(event Custom|WeaponFire
  (bind _self self)
  (bind _turret (Variables|Default|GetTurret))
  (bind _firepoint (Variables|/Game/Blueprints/ai/BotTurret.BotTurret_C|GetFirePoint _turret))
  (bind _returnvalue (Transformation|GetWorldTransform _firepoint))
  (Game|SpawnActorfromClass (Variables|Default|GetProjectileType) (Math|Transform|MakeTransform (.location _returnvalue) (.rotation _returnvalue) "3.000000,3.000000,3.000000") "Undefined" _self _self self)
  (Development|PrintString "firing")
  (Variables|Default|SetWeaponCooldown true)
  (Utilities|Time|SetTimerbyEvent (delegate Custom|ResetFire) (Variables|Default|GetFireDelay)))

(event Custom|TargetDied
  (CallFunction|GetNewTarget))

(event Custom|ResetFire
  (Variables|Default|SetWeaponCooldown false))

(event Custom|PostSpawn
  (Rendering|Components|Decal|SetDecalMaterial (Variables|Default|GetDecal) (Utilities|Select :Index (.playerteam (Variables|Default|Gettankinfo)) :Option%200 "/Game/CustomAssets/Materials/Decals/M_RedTeamCircle.M_RedTeamCircle" :Option%201 "/Game/CustomAssets/Materials/Decals/M_BlueTeamCircle.M_BlueTeamCircle" :Option%202 "/Game/CustomAssets/Materials/Decals/M_GreenTeamCircle.M_GreenTeamCircle" :Option%203 "/Game/CustomAssets/Materials/Decals/M_YellowTeamCircle.M_YellowTeamCircle")))

(event EventSetPlayerInfo
  (params (playerInfo :type Player%20Info%20Structure))
  (Variables|Default|Settankinfo playerInfo)
  (CallFunction|PostSpawn))

(event Game|Damage|EventAnyDamage
  (params (Damage :type Float%20%28single-precision%29) (DamageType :type Damage%20Type%20Object%20Reference) (InstigatedBy :type Controller%20Object%20Reference) (DamageCauser :type Actor%20Object%20Reference))
  (bind _asbp_projectile_base (Utilities|Casting|CastToBP_ProjectileBase DamageCauser))
  (if (not (== self (Variables|/Game/Blueprints/Tank/Projectiles/BP_ProjectileBase.BP_ProjectileBase_C|GetBP_TankRef _asbp_projectile_base)))
    (bind _output_get (Variables|Default|SetCurrentHealth (- (Variables|Default|GetCurrentHealth) Damage)))
    (if (<= _output_get 0.0)
      (bind _asdeath_match_game_mode (Utilities|Casting|CastToDeathMatchGameMode (Game|GetGameMode)))
      (Default|RespawnBot _asdeath_match_game_mode self)
      (bind _info (Class|ICharacterInterface|GetPlayerInfo(Message) (Variables|Default|GetLastAttackedBy)))
      (Default|ScorePoint _asdeath_match_game_mode (.playerteam _info))
      (else
        (if (Utilities|IsValid InstigatedBy)
          (Variables|Default|SetLastAttackedBy (Pawn|GetControlledPawn InstigatedBy))
          (else
            (bind _output_get_2 (Variables|Default|SetLastAttackedBy (Variables|/Game/Blueprints/Tank/Projectiles/BP_ProjectileBase.BP_ProjectileBase_C|GetBP_TankRef _asbp_projectile_base)))))
        (if (!= _output_get_2 (Variables|Default|GetCurrentTarget))
          (Variables|Default|SetCurrentTarget (Variables|Default|GetLastAttackedBy)))))))

(event EventTick
  (params (DeltaSeconds :type Float%20%28single-precision%29))
  (bind _pathtotarget (Variables|Default|GetPathToTarget))
  (if (Utilities|IsValid (Variables|Default|GetCurrentTarget))
    (CallFunction|GetPathtoTarget)
    (bind _lineofsight (CallFunction|LineOfSight))
    (if _lineofsight
      (CallFunction|ShouldtheBodyRotate)
      (if (>= (Variables|Default|GetDistanceTurned) (Variables|Default|GetFireArc))
        (CallFunction|RotatetoFaceTarget))
      (bind _distance (CallFunction|GetDistancetoCurrentTarget))
      (if (< _distance (Variables|Default|GetStoppingDistance))
        (if (not (Variables|Default|GetWeaponCooldown))
          (CallFunction|WeaponFire)
          (Utilities|Time|SetTimerbyEvent (delegate Custom|WeaponFire) (Variables|Default|GetFireDelay)))
        (else
          (CallFunction|RotatetoFacePath)
          (Physics|AddForce (Variables|Default|GetStaticMesh) (* (Math|Vector|GetForwardVector (Variables|Default|GetStaticMesh)) (Variables|Default|GetSpeed)) "None" true)))
      (else
        (CallFunction|RotatetoFacePath)
        (Physics|AddForce (Variables|Default|GetStaticMesh) (* (Math|Vector|GetForwardVector (Variables|Default|GetStaticMesh)) (Variables|Default|GetSpeed)) "None" true)
        (Utilities|IsCurrentPathnodeValid _pathtotarget
          (:true
            (if (<= (Math|Vector|VectorLength (- (Transformation|GetActorLocation) (Utilities|Array|Get(acopy) _pathtotarget (Variables|Default|GetPathId)))) 5e+02)
              (bind _result (Math|Integer|IncrementInt (Variables|Default|GetPathId))
                (:%20%20
                  (Variables|Default|SetPathId _result)
                  (if (> (Variables|Default|GetPathId) (Utilities|Array|Length (Variables|Default|GetPathToTarget)))
                    (Variables|Default|SetPathId 0)))))))))
    (else
      (CallFunction|GetNewTarget))))

(event EventBeginPlay
  (bind _returnvalue (Game|SpawnActorfromClass "/Game/Blueprints/ai/BotTurret.BotTurret_C" (Transformation|GetWorldTransform (Variables|Default|GetTurretSpawn)) "Undefined" 0 0))
  (bind _output_get (Variables|Default|SetTurret _returnvalue))
  (Variables|/Game/Blueprints/ai/BotTurret.BotTurret_C|SetTank _output_get self)
  (Variables|Default|SetCurrentHealth (Variables|Default|GetMaxHealth)))

(event EventDestroyed
  (Development|PrintString "tank killed"))

(fn ConstructionScript)

(fn GetDistancetoCurrentTarget
  (bind _currenttarget (Variables|Default|GetCurrentTarget))
  (if (Utilities|IsValid _currenttarget)
    (return (Math|Vector|VectorLength (- (Transformation|GetActorLocation _currenttarget) (Transformation|GetActorLocation))))))

(fn LineOfSight
  (bind _currenttarget (Variables|Default|GetCurrentTarget))
  (if (Utilities|IsValid _currenttarget)
    (bind _outhit (Collision|LineTraceByChannel (Transformation|GetActorLocation) (Transformation|GetActorLocation _currenttarget) "TraceTypeQuery1" false 0 "None"))
    (if (== (.HitActor (Collision|BreakHitResult _outhit)) (Variables|Default|GetCurrentTarget))
      (Variables|Default|SetLastKnownDirection (.Location (Collision|BreakHitResult _outhit))))
    (return (== (.HitActor (Collision|BreakHitResult _outhit)) (Variables|Default|GetCurrentTarget)))))

(fn RotatetoFaceTarget
  (Transformation|SetActorRelativeRotation (Math|Rotator|FindLookatRotation (Transformation|GetActorLocation) (Transformation|GetActorLocation (Variables|Default|GetCurrentTarget)))))

(fn GetPathtoTarget
  (bind _currenttarget (Variables|Default|GetCurrentTarget))
  (bind _outactors (Actor|GetAllActorsOfClass "/Script/NavigationSystem.NavMeshBoundsVolume"))
  (if (Utilities|IsValid _currenttarget)
    (bind _returnvalue (Class|NavigationSystemV1|FindPathtoLocationSynchronously (Utilities|Array|Get(acopy) _outactors) (Transformation|GetActorLocation) (Transformation|GetActorLocation _currenttarget) 0 0))
    (bind _output_get (Variables|Default|SetPathToTarget (Variables|/Script/NavigationSystem.NavigationPath|GetPathPoints _returnvalue)))
    (Utilities|Array|RemoveIndex _output_get)
    (Variables|Default|SetPathId 0)
    (for _array_element _output_get
      (Rendering|Debug|DrawDebugSphere _array_element 5e+01 12 "(R=1.000000,G=0.000000,B=0.044905,A=1.000000)" 0.0 5e+01))))

(fn RotatetoFacePath
  (bind _pathtotarget (Variables|Default|GetPathToTarget))
  (bind _pathid (Variables|Default|GetPathId))
  (bind _output (Utilities|Array|Get(acopy) _pathtotarget _pathid))
  (Utilities|IsCurrentPathnodeValid _pathtotarget
    (:true
      (Transformation|SetActorRelativeRotation (Math|Rotator|FindLookatRotation (Transformation|GetActorLocation) (Math|Vector|MakeVector (.x _output) (.y _output) (.z (Transformation|GetActorLocation))))))))

(fn RotateTurrettoFaceTarget
  (bind _turret (Variables|Default|GetTurret))
  (bind _returnvalue (Transformation|GetActorLocation _turret))
  (Transformation|SetActorRelativeRotation _turret (Math|Rotator|FindLookatRotation _returnvalue (- (Transformation|GetActorLocation (Variables|Default|GetCurrentTarget)) _returnvalue))))

(fn ShouldtheBodyRotate
  (Variables|Default|SetDistanceTurned (Class|KismetMathLibrary|DegAcos (Math|Vector|DotProduct (Transformation|GetActorForwardVector) (Math|Vector|GetForwardVector (Variables|/Game/Blueprints/ai/BotTurret.BotTurret_C|GetStaticMesh (Variables|Default|GetTurret)))))))

(fn GetNewTarget
  (if (not (Utilities|IsValid (Variables|Default|GetCurrentTarget)))
    (bind _outactors (Actor|GetAllActorsOfClass "/Game/Blueprints/Tank/BP_Tank.BP_Tank_C"))
    (for _array_element _outactors
      (Utilities|Array|Add (LocalVariables|GetAllPosibleTargets) _array_element))
    (bind _outactors_2 (Actor|GetAllActorsOfClass "/Temp/Diff/temp-9f633c3e8155017e4f70b0fb7f5e745f51602120-DeathMatchBot.DeathMatchBot_C"))
    (for _array_element_2 _outactors_2
      (if (!= _array_element_2 self)
        (Utilities|Array|Add (LocalVariables|GetAllPosibleTargets) _array_element_2)))
    (Variables|Default|SetCurrentTarget (Utilities|Array|Get(acopy) (LocalVariables|GetAllPosibleTargets) (Math|Random|RandomInteger (Utilities|Array|Length (LocalVariables|GetAllPosibleTargets)))))))

(fn GetPlayerInfo
  (return (Variables|Default|Gettankinfo)))

(fn GetSelfandPawn
  (return 0 0))