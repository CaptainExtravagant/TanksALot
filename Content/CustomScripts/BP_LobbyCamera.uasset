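; Menu camera actor that moves between main menu, options and lobby viewpoints in response to Settings, Play and Return button events.
; It snaps to the main menu transform on BeginPlay, then timelines lerp it to the options or lobby transform.
; Return plays the matching timeline in reverse, chosen by a FromLobby flag.
; A Moving flag tracks transitions, while GetCurrentMenuState always returns the first enum value.
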(event Custom|TransitionFromLobby
  ;[1 1 1] OptionsTransition
  (Variables|Default|SetNewTime 1.0)
  (Variables|Default|SetMoving true)
  (bind _completion (Timeline|LobbyMotion ReverseFromEnd)
    (:Update
      (Transformation|SetWorldTransform (Variables|Default|GetCamera) (Math|Transform|Lerp(Transform) (Variables|Default|GetMainMenuPosition) (Variables|Default|GetLobbyMenuPosition) _completion) false false))
    (:Finished
      (Variables|Default|SetMoving false))))

(event Custom|TransitionToLobby
  ;[1 1 1] OptionsTransition
  (Variables|Default|SetNewTime 0.0)
  (Variables|Default|SetMoving true)
  (bind _completion (Timeline|LobbyMotion PlayFromStart)
    (:Update
      (Transformation|SetWorldTransform (Variables|Default|GetCamera) (Math|Transform|Lerp(Transform) (Variables|Default|GetMainMenuPosition) (Variables|Default|GetLobbyMenuPosition) _completion) false false))
    (:Finished
      (Variables|Default|SetMoving false))))

(event Custom|TransitionToOptions
  ;[1 1 1] OptionsTransition
  (Variables|Default|SetNewTime 0.0)
  (Variables|Default|SetMoving true)
  (bind _completion (Timeline|OptionsMotion PlayFromStart)
    (:Update
      (Transformation|SetWorldTransform (Variables|Default|GetCamera) (Math|Transform|Lerp(Transform) (Variables|Default|GetMainMenuPosition) (Variables|Default|GetOptionsMenuPosition) _completion) false false))
    (:Finished
      (Variables|Default|SetMoving false))))

(event Custom|TransitionFromOptions
  ;[1 1 1] OptionsTransition
  (Variables|Default|SetNewTime 1.0)
  (Variables|Default|SetMoving true)
  (bind _completion (Timeline|OptionsMotion ReverseFromEnd)
    (:Update
      (Transformation|SetWorldTransform (Variables|Default|GetCamera) (Math|Transform|Lerp(Transform) (Variables|Default|GetMainMenuPosition) (Variables|Default|GetOptionsMenuPosition) _completion) false false))
    (:Finished
      (Variables|Default|SetMoving false))))

(event EventBeginPlay
  (Transformation|SetWorldTransform (Variables|Default|GetCamera) (Variables|Default|GetMainMenuPosition) false false))

(event Collision|EventActorBeginOverlap
  (params (OtherActor :type Actor%20Object%20Reference)))

(event EventTick
  (params (DeltaSeconds :type Float%20%28single-precision%29)))

(event EventReturnButton
  (params (FromLobby? :type Boolean))
  (if FromLobby?
    (CallFunction|TransitionfromLobby)
    (else
      (CallFunction|TransitionfromOptions))))

(event EventSettingsButton
  (CallFunction|TransitiontoOptions))

(event EventPlayButton
  (CallFunction|TransitiontoLobby))

(fn ConstructionScript)

(fn GetCurrentMenuState
  (return "NewEnumerator0"))